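; Closet door for the closet rhythm minigame that the player slams shut to hit notes.
; Tick watches the door's yaw and fires once per close with sound and emissive flash, either calling Slammed on the note manager or, during play, scoring a hit or miss.
; Overlap boxes track the current note and grade hit quality, feeding the manager's streak; hits also spawn floating text, pulse pooled notes and trigger right-hand haptics.
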(event OnComponentBeginOverlap(BC_NoteCollision)
  (params (OverlappedComponent :type Primitive%20Component%20Object%20Reference) (OtherActor :type Actor%20Object%20Reference) (OtherComp :type Primitive%20Component%20Object%20Reference) (OtherBodyIndex :type Integer) (bFromSweep :type Boolean) (SweepResult :type Hit%20Result%20Structure%20%28by%20ref%29))
  (bind _asbp_note (Utilities|Casting|CastToBP_Note OtherActor))
  (Utilities|IsValid (Variables|Default|GetOverlappingNote)
    (:Is%20Valid
      (Default|DisableNote _asbp_note))
    (:Is%20Not%20Valid
      (Variables|Default|SetOverlappingNote _asbp_note))))

(event OnComponentEndOverlap(BC_NoteCollision)
  (params (OverlappedComponent :type Primitive%20Component%20Object%20Reference) (OtherActor :type Actor%20Object%20Reference) (OtherComp :type Primitive%20Component%20Object%20Reference) (OtherBodyIndex :type Integer))
  (if (== (Variables|Default|GetOverlappingNote) OtherActor)
    (Default|DisableAfterDelay (Variables|Default|GetOverlappingNote) 1.0)
    (Variables|Default|SetOverlappingNote 0)
    (Default|EndStreak (Variables|Default|GetNoteManager))))

(event Custom|HitNote
  (Utilities|FlowControl|Sequence
    (:then_0
      ;[1 1 1] CHECK FOR QUALITY OF THE NOTE HIT
      (Variables|Default|SetHitQuality "NewEnumerator3")
      (if (Collision|IsOverlappingActor (Variables|Default|GetBC_BadHit) (Variables|Default|GetOverlappingNote) :!class /Script/Engine.PrimitiveComponent)
        (Variables|Default|SetHitQuality "NewEnumerator0")))
    (:then_1
      (if (Collision|IsOverlappingActor (Variables|Default|GetBC_GoodHit) (Variables|Default|GetOverlappingNote) :!class /Script/Engine.PrimitiveComponent)
        (Variables|Default|SetHitQuality "NewEnumerator1")))
    (:then_2
      (if (Collision|IsOverlappingActor (Variables|Default|GetBC_PerfectHit) (Variables|Default|GetOverlappingNote) :!class /Script/Engine.PrimitiveComponent)
        (Variables|Default|SetHitQuality "NewEnumerator2")))
    (:then_3
      (Default|AddtoStreak (Variables|Default|GetNoteManager) (Variables|Default|GetHitQuality))
      (Default|DestroyNote (Variables|Default|GetOverlappingNote))
      (Variables|Default|SetOverlappingNote 0))
    (:then_4
      (Game|SpawnActorfromClass "/Game/Blueprints/Minigames/Mole/BP_FloatingTextRenderer_Ryhtm.BP_FloatingTextRenderer_Ryhtm_C" (Math|Transform|MakeTransform (Transformation|GetWorldLocation (Variables|Default|GetA_FloatingTextSpawnLocation)) "0, 0, 0" "1,1,1") "AlwaysSpawn" 0 (Variables|Default|GetHitQuality) 0)
      (CallFunction|PulseAllSmalNotes))
    (:then_5
      (Class|PlayerController|PlayHapticEffect (Game|GetPlayerController 0) "/Game/Blueprints/Gameplay/HF_Standard.HF_Standard" "Right" 1.0 false))))

(event Custom|Miss
  (Variables|Default|SetHitQuality "NewEnumerator3")
  (Default|AddtoStreak (Variables|Default|GetNoteManager) (Variables|Default|GetHitQuality)))

(event EventBeginPlay
  (bind _pdoor (Variables|Default|GetpDoor))
  (Utilities|FlowControl|Sequence
    (:then_0
      (bind _outactors (Actor|GetAllActorsOfClass "/Game/Blueprints/Minigames/ClosetRythm/BP_Notemanager.BP_Notemanager_C"))
      (bind _output_get (Variables|Default|SetNoteManager (Utilities|Array|Get(acopy) _outactors)))
      (Utilities|FlowControl|Delay 0.0)
      (Variables|/Game/Blueprints/Minigames/ClosetRythm/BP_Notemanager.BP_Notemanager_C|SetHasSlammed _output_get false))
    (:then_1
      (bind _returnvalue (Rendering|Material|CreateDynamicMaterialInstance _pdoor 0 (Rendering|Material|GetMaterial _pdoor 0) "None" :!class /Script/Engine.PrimitiveComponent))
      (Variables|Default|SetDynMaterial _returnvalue))
    (:then_2
      (Rendering|SetVisibility (Variables|Default|GetTR_Tip) true true))))

(event EventTick
  (params (DeltaSeconds :type Float%20%28single-precision%29))
  (Utilities|FlowControl|Sequence
    (:then_0
      (if (<= (.yaw (Variables|/Script/Engine.SceneComponent|GetRelativeRotation (Variables|Default|GetpDoorRotator))) (.yaw (Variables|/Script/Engine.SceneComponent|GetRelativeRotation (Variables|Default|GetA_ClosedRotation))))
        (Utilities|FlowControl|DoOnce true :!label _label
          (:Completed
            (Utilities|FlowControl|Sequence
              (:then_0
                (if (Variables|/Game/Blueprints/Minigames/ClosetRythm/BP_Notemanager.BP_Notemanager_C|GetIsPlaying (Variables|Default|GetNoteManager))
                  (if (Utilities|IsValid (Variables|Default|GetOverlappingNote))
                    (CallFunction|HitNote)
                    (else
                      (CallFunction|Miss)))
                  (else
                    (Default|Slammed (Variables|Default|GetNoteManager)))))
              (:then_1
                (bind _emissivevalue (Timeline|Timeline_0 PlayFromStart)
                  (:Update
                    (CallFunction|SetEmissive _emissivevalue))))
              (:then_2
                (Audio|PlaySoundatLocation "/Game/Audio/SFX/SFX_ClosetCloseSound_Cue.SFX_ClosetCloseSound_Cue" (Transformation|GetActorLocation) "0, 0, 0" 0.1 (Math|Random|RandomFloatinRange 0.8 1.2) 0.0 0 0 0)))))
        (else
          (goto _label Reset))))
    (:then_1
      (if (Variables|/Game/Blueprints/Minigames/ClosetRythm/BP_Notemanager.BP_Notemanager_C|GetIsPlaying (Variables|Default|GetNoteManager))
        (Utilities|FlowControl|DoOnce false
          (:Completed
            (Rendering|SetVisibility (Variables|Default|GetTR_Tip) false true)))))))

(fn ConstructionScript
  (Variables|Default|SetbHoldOnForever true))

(fn SetEmissive
  (params (NewEmissiveValue :type Float%20%28single-precision%29))
  (Rendering|Material|SetScalarParameterValue (Variables|Default|GetDynMaterial) "EmissiveIntensity" NewEmissiveValue :!class /Script/Engine.MaterialInstanceDynamic))

(fn PulseAllSmalNotes
  (for _array_element (Variables|/Game/Blueprints/Minigames/ClosetRythm/BP_Notemanager.BP_Notemanager_C|GetClosetSlamNotesObjectPool (Variables|Default|GetNoteManager))
    (Utilities|IsValid _array_element
      (:Is%20Valid
        (Default|Pulse _array_element)))))