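; Manager for the closet rhythm minigame, which starts once both closets are triggered (slap and slam) and can be played once.
; Tick spawns notes from two pre-spawned object pools on per-lane delay arrays, with velocities aimed at each closet.
; Hit quality updates text counters and a streak that drives note and closet emissive glow.
; When time runs out, the player's hands break, info unlocks and the death scene loads after a fade.
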(event Custom|GameOver
  (Audio|PlaySound2D "/Game/Audio/SFX/SFX_HandBreaking.SFX_HandBreaking" 0.5 1.0 0.0 0 0)
  (Rendering|SetVisibility (Variables|Default|GetSkeletalMesh) true false)
  (bind _asbp_game_instance (Utilities|Casting|CastToBP_GameInstance (Game|GetGameInstance)))
  (Default|Breakhands (Variables|/Game/Blueprints/BP_GameInstance.BP_GameInstance_C|GetBasePawn _asbp_game_instance))
  (Variables|Default|SetIsPlaying false)
  (Variables|Default|SetHasPlayed true)
  (bind _asbp_game_instance_2 (Utilities|Casting|CastToBP_GameInstance (Game|GetGameInstance)))
  (Default|UnlockInfo _asbp_game_instance_2 "NewEnumerator2")
  (Default|SetSpringText (Variables|/Game/Blueprints/BP_GameInstance.BP_GameInstance_C|GetBasePawn _asbp_game_instance_2) "YOUR HAND GOT 
HIT BY THE CLOSET" 1.0)
  (Utilities|FlowControl|Delay 1e+01)
  (bind _asbp_game_instance_3 (Utilities|Casting|CastToBP_GameInstance (Game|GetGameInstance)))
  (Variables|/Game/Blueprints/BP_GameInstance.BP_GameInstance_C|SetLevelLoadOptions _asbp_game_instance_3 "Rythm")
  (CameraFades|StartCameraFade (Game|GetPlayerCameraManager 0) 0.0 1.0 (Variables|/Game/Blueprints/BP_GameInstance.BP_GameInstance_C|GetFadeTime _asbp_game_instance_3) "(R=1.000000,G=1.000000,B=1.000000,A=1.000000)" false true)
  (Utilities|FlowControl|Delay (Variables|/Game/Blueprints/BP_GameInstance.BP_GameInstance_C|GetFadeTime _asbp_game_instance_3))
  (Game|OpenLevel(byName) "MAP_PlayerDeadScene"))

(event Custom|StartPlaying
  (Utilities|FlowControl|Delay 2.5)
  (Audio|PlaySound2D "/Game/Audio/AMB/AMB_Rythmgame.AMB_Rythmgame" 0.1 1.0 0.0 0 0)
  (Rendering|SetVisibility (Variables|Default|GetTR_Info) false true)
  (Rendering|SetVisibility (Variables|Default|GetSC_Hits) true true)
  (Rendering|SetVisibility (Variables|Default|GetTR_StreakStatic) true true))

(event EventBeginPlay
  (Utilities|FlowControl|Sequence
    (:then_0
      (bind _outactors (Actor|GetAllActorsOfClass "/Game/Blueprints/Minigames/ClosetRythm/BP_ClosetSlap.BP_ClosetSlap_C"))
      (Variables|ClosetSlap|SetClosetSlap (Utilities|Array|Get(acopy) _outactors))
      (bind _outactors_2 (Actor|GetAllActorsOfClass "/Game/Blueprints/Minigames/ClosetRythm/BP_ClosetSlam.BP_ClosetSlam_C"))
      (Variables|ClosetSlam|SetClosetSlam (Utilities|Array|Get(acopy) _outactors_2)))
    (:then_1
      (ObjectPooling|ExpandClosetSlapNoteObjectPool 20)
      (ObjectPooling|ExpandClosetSlamNoteObjectPool 20))
    (:then_2
      (Rendering|SetVisibility (Variables|Default|GetTR_Info) true true)
      (Rendering|SetVisibility (Variables|Default|GetSC_Hits) false true)
      (Rendering|SetVisibility (Variables|Default|GetTR_StreakStatic) false true)
      (Rendering|SetVisibility (Variables|Default|GetSkeletalMesh) false false))))

(event EventTick
  (params (DeltaSeconds :type Float%20%28single-precision%29))
  (if (Variables|Default|GetIsPlaying)
    (Variables|Default|SetElapsedTime (+ DeltaSeconds (Variables|Default|GetElapsedTime)))
    (if (< (Variables|Default|GetElapsedTime) (Variables|Default|GetGameTime))
      (Utilities|FlowControl|Sequence
        (:then_0
          ;[1 1 1] SPAWN A NOTE EVERY COUPLE OF SECONDS
          (if (Variables|ClosetSlap|GetbClosetSlapNotesAvailable)
            (Utilities|FlowControl|Delay (Utilities|Array|Get(acopy) (Variables|ClosetSlap|GetClosetSlapNoteSpawnDelay) (Variables|ClosetSlap|GetClosetSlapIndex)))
            (CallFunction|SpawnClosetSlapNote)))
        (:then_1
          (if (Variables|ClosetSlam|GetbClosetSlamNotesAvailable)
            (Utilities|FlowControl|Delay (Utilities|Array|Get(acopy) (Variables|ClosetSlam|GetClosetSlamNoteSpawnDelay) (Variables|ClosetSlam|GetClosetSlamIndex)))
            (CallFunction|SpawnClosetSlamNote)))
        (:then_2
          (Development|PrintString (Utilities|String|ToString(Integer) (ObjectPooling|ClosetSlapNotesActive)) true true "(R=0.000000,G=0.660000,B=1.000000,A=1.000000)" 0.0)))
      (else
        (CallFunction|GameOver)))))

(fn ConstructionScript)

(fn AddtoStreak
  (params (hitQuality :type eHITQUALITY%20Enum :default "NewEnumerator3"))
  (if (Utilities|Enum|NotEqual(Enum) hitQuality "NewEnumerator3")
    (Utilities|FlowControl|Sequence
      (:then_0
        (Math|Integer|IncrementInt (Variables|Streak|GetStreak)
          (:%20%20
            (if (> (Variables|Streak|GetStreak) (Variables|Streak|GetBestStreak))
              (Variables|Streak|SetBestStreak (Variables|Streak|GetStreak)))
            (Rendering|Components|TextRender|SetText (Variables|Default|GetTR_StreakCount) (Utilities|Text|ToText(Integer) (Variables|Streak|GetStreak)))
            (Rendering|Components|TextRender|SetText (Variables|Default|GetTR_BestStreak) (Utilities|Text|ToText(Integer) (Variables|Streak|GetBestStreak)))
            (CallFunction|UpdateEmissiveIntensityOfNotes))))
      (:then_1
        (switch Utilities|FlowControl|Switch|SwitchoneHITQUALITY hitQuality :!label _label
          (:NewEnumerator3
            (bind _result (Math|Integer|IncrementInt (Variables|Streak|GetMisses))
              (:%20%20
                (Rendering|Components|TextRender|SetText (Variables|Default|GetTR_MissesCount) (Utilities|Text|ToText(Integer) _result)))))
          (:NewEnumerator0
            (bind _result_2 (Math|Integer|IncrementInt (Variables|Streak|GetBadHits))
              (:%20%20
                (Rendering|Components|TextRender|SetText (Variables|Default|GetTR_BadsCount) (Utilities|Text|ToText(Integer) _result_2)))))
          (:NewEnumerator1
            (bind _result_3 (Math|Integer|IncrementInt (Variables|Streak|GetGoodHits))
              (:%20%20
                (Rendering|Components|TextRender|SetText (Variables|Default|GetTR_GoodsCount) (Utilities|Text|ToText(Integer) _result_3)))))
          (:NewEnumerator2
            (bind _result_4 (Math|Integer|IncrementInt (Variables|Streak|GetPrefectHits))
              (:%20%20
                (Rendering|Components|TextRender|SetText (Variables|Default|GetTR_PerfectsCount) (Utilities|Text|ToText(Integer) _result_4))))))))
    (else
      (CallFunction|EndStreak)
      (goto _label))))

(fn EndStreak
  (bind _output_get (Variables|Streak|SetStreak 0))
  (Rendering|Components|TextRender|SetText (Variables|Default|GetTR_StreakCount) (Utilities|Text|ToText(Integer) _output_get))
  (CallFunction|UpdateEmissiveIntensityOfNotes))

(fn SpawnClosetSlapNote
  (bind _availablenote (ObjectPooling|GetAvailableClosetSlapNote))
  (Utilities|IsValid _availablenote
    (:Is%20Valid
      (Default|EnableNote _availablenote)
      (Transformation|SetWorldLocation (Variables|/Game/Blueprints/Minigames/ClosetRythm/BP_Note.BP_Note_C|GetStaticMesh _availablenote) (Transformation|GetWorldLocation (Variables|Default|GetA_ClosetSlapNodeSpawn)) false true)
      (Rendering|Material|SetScalarParameterValue (Variables|/Game/Blueprints/Minigames/ClosetRythm/BP_Note.BP_Note_C|GetDynMaterial _availablenote) "EmissiveIntensity" 1.0 :!class /Script/Engine.MaterialInstanceDynamic)
      (Transformation|SetWorldScale3D (Variables|/Game/Blueprints/Minigames/ClosetRythm/BP_Note.BP_Note_C|GetStaticMesh _availablenote) (Variables|/Game/Blueprints/Minigames/ClosetRythm/BP_Note.BP_Note_C|GetScale _availablenote))
      (bind _result (Math|Integer|IncrementInt (Variables|ClosetSlap|GetClosetSlapIndex))
        (:%20%20
          (if (>= _result (Utilities|Array|Length (Variables|ClosetSlap|GetClosetSlapNoteSpawnDelay)))
            (Variables|ClosetSlap|SetClosetSlapIndex 0)
            (else
              (Variables|ClosetSlap|SetbClosetSlapNotesAvailable true))))))))

(fn GetAvailableClosetSlapNote
  (for _array_element (Variables|ClosetSlap|GetClosetSlapNotesObjectPool)
    (if (not (Variables|/Game/Blueprints/Minigames/ClosetRythm/BP_Note.BP_Note_C|GetbIsActive _array_element))
      (return _array_element))))

(fn ExpandClosetSlapNoteObjectPool
  (params (NumberOfObjectsToSpawn :type Integer))
  ;[1 1 1] SPAWN NOTES FOR THE OBJECT POOL
  (for _index (range 0 NumberOfObjectsToSpawn)
    (bind _returnvalue (Game|SpawnActorfromClass "/Game/Blueprints/Minigames/ClosetRythm/BP_ClosetSlapNote.BP_ClosetSlapNote_C" (Transformation|GetWorldTransform (Variables|Default|GetA_ClosetSlapNodeSpawn)) "Undefined" 0 0))
    (Utilities|Array|Add (Variables|ClosetSlap|GetClosetSlapNotesObjectPool) _returnvalue)
    (Default|DisableNote _returnvalue)
    (Variables|/Game/Blueprints/Minigames/ClosetRythm/BP_Note.BP_Note_C|SetVelocity _returnvalue (* (Utilities|VelocityTowardsSlapCloset) (Variables|General|GetNoteSpeed)))))

(fn ClosetSlapNotesActive
  (for _array_element (Variables|ClosetSlap|GetClosetSlapNotesObjectPool)
    (if (Variables|/Game/Blueprints/Minigames/ClosetRythm/BP_Note.BP_Note_C|GetbIsActive _array_element)
      (Math|Integer|IncrementInt (LocalVariables|GetCount))))
  (return (LocalVariables|GetCount)))

(fn GetAvailableCloseSlamNote
  (for _array_element (Variables|ClosetSlam|GetClosetSlamNotesObjectPool)
    (if (not (Variables|/Game/Blueprints/Minigames/ClosetRythm/BP_Note.BP_Note_C|GetbIsActive _array_element))
      (return _array_element))))

(fn ExpandClosetSlamNoteObjectPool
  (params (NumberOfObjectsToSpawn :type Integer))
  ;[1 1 1] SPAWN NOTES FOR THE OBJECT POOL
  (for _index (range 0 NumberOfObjectsToSpawn)
    (bind _returnvalue (Game|SpawnActorfromClass "/Game/Blueprints/Minigames/ClosetRythm/BP_ClosetSlamNote.BP_ClosetSlamNote_C" (Transformation|GetWorldTransform (Variables|Default|GetA_ClosetSlamNodeSpawn)) "Undefined" 0 0))
    (Utilities|Array|Add (Variables|ClosetSlam|GetClosetSlamNotesObjectPool) _returnvalue)
    (Default|DisableNote _returnvalue)
    (Variables|/Game/Blueprints/Minigames/ClosetRythm/BP_Note.BP_Note_C|SetVelocity _returnvalue (* (Utilities|VelocityTowardsSlamCloset) (Variables|General|GetNoteSpeed)))))

(fn ClosetSlamNotesActive
  (for _array_element (Variables|ClosetSlam|GetClosetSlamNotesObjectPool)
    (if (Variables|/Game/Blueprints/Minigames/ClosetRythm/BP_Note.BP_Note_C|GetbIsActive _array_element)
      (Math|Integer|IncrementInt (LocalVariables|GetCount))))
  (return (LocalVariables|GetCount)))

(fn SpawnClosetSlamNote
  (bind _availablenote (ObjectPooling|GetAvailableCloseSlamNote))
  (Utilities|IsValid _availablenote
    (:Is%20Valid
      (Default|EnableNote _availablenote)
      (Transformation|SetWorldLocation (Variables|/Game/Blueprints/Minigames/ClosetRythm/BP_Note.BP_Note_C|GetStaticMesh _availablenote) (Transformation|GetWorldLocation (Variables|Default|GetA_ClosetSlamNodeSpawn)) false true)
      (bind _result (Math|Integer|IncrementInt (Variables|ClosetSlam|GetClosetSlamIndex))
        (:%20%20
          (if (>= _result (Utilities|Array|Length (Variables|ClosetSlap|GetClosetSlapNoteSpawnDelay)))
            (Variables|ClosetSlam|SetClosetSlamIndex 0)
            (else
              (Variables|ClosetSlam|SetbClosetSlamNotesAvailable true))))))))

(fn Slapped
  (if (and (not (Variables|Default|GetIsPlaying)) (not (Variables|Default|GetHasPlayed)))
    (Variables|Default|SetHasSlapped true)
    (bind _output_get (Variables|Default|SetIsPlaying (and (Variables|Default|GetHasSlammed) (Variables|Default|GetHasSlapped))))
    (if _output_get
      (CallFunction|StartPlaying))))

(fn Slammed
  (if (and (not (Variables|Default|GetIsPlaying)) (not (Variables|Default|GetHasPlayed)))
    (Variables|Default|SetHasSlammed true)
    (bind _output_get (Variables|Default|SetIsPlaying (and (Variables|Default|GetHasSlammed) (Variables|Default|GetHasSlapped))))
    (if _output_get
      (CallFunction|StartPlaying))))

(fn UpdateEmissiveIntensityOfNotes
  (Utilities|FlowControl|Sequence
    (:then_0
      (for _array_element (Variables|ClosetSlap|GetClosetSlapNotesObjectPool)
        (Default|SetEmissive _array_element (Utilities|GetEmissiveBasedonStreak))))
    (:then_1
      (for _array_element_2 (Variables|ClosetSlam|GetClosetSlamNotesObjectPool)
        (Default|SetEmissive _array_element_2 (Utilities|GetEmissiveBasedonStreak))))
    (:then_2
      (Default|SetEmissive (Variables|ClosetSlap|GetClosetSlap) (Utilities|GetEmissiveBasedonStreak)))
    (:then_3
      (Default|SetEmissive (Variables|ClosetSlam|GetClosetSlam) (Utilities|GetEmissiveBasedonStreak)))))

(fn GetTotalTime
  (Utilities|FlowControl|Sequence
    (:then_0
      (for _array_element (Variables|ClosetSlap|GetClosetSlapNoteSpawnDelay)
        (LocalVariables|SetSlapTotalTime (+ _array_element (LocalVariables|GetSlapTotalTime))))
      (for _array_element_2 (Variables|ClosetSlam|GetClosetSlamNoteSpawnDelay)
        (LocalVariables|SetSlamTotalTime (+ _array_element_2 (LocalVariables|GetSlamTotalTime)))))
    (:then_1
      (if (> (LocalVariables|GetSlapTotalTime) (LocalVariables|GetSlamTotalTime))
        (return (LocalVariables|GetSlapTotalTime))
        (else
          (return (LocalVariables|GetSlamTotalTime)))))))