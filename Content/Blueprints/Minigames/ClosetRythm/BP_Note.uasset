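; BP_Note is a note actor for the closet rhythm minigame that moves along a velocity while active.
; Tick sweeps the mesh forward, and EnableNote and DisableNote toggle movement and visibility instead of destroying the actor.
; DestroyNote spawns a collect particle before disabling, and DisableAfterDelay disables it on a timer.
; A pulse timeline animates scale and dynamic material emissive, then restores the stored streak intensity.
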(event Custom|DestroyNote
  (Effects|SpawnEmitteratLocation "/Game/FX/P_Pill_collected.P_Pill_collected" (Transformation|GetActorLocation))
  (CallFunction|DisableNote))

(event Custom|DisableAfterDelay
  (params (DisableAfter :type Float%20%28single-precision%29))
  (Utilities|FlowControl|Delay DisableAfter)
  (CallFunction|DisableNote))

(event Custom|Pulse
  (bind (_direction _emissiveboost _scale) (Timeline|PulseTimeline PlayFromStart)
    (:Update
      (Rendering|Material|SetScalarParameterValue (Variables|Default|GetDynMaterial) "EmissiveIntensity" _emissiveboost :!class /Script/Engine.MaterialInstanceDynamic)
      (Transformation|SetWorldScale3D (Variables|Default|GetStaticMesh) (Math|Conversions|ToVector(Float) _scale)))
    (:Finished
      (Rendering|Material|SetScalarParameterValue (Variables|Default|GetDynMaterial) "EmissiveIntensity" (Variables|Default|GetEmissiveStreakVal) :!class /Script/Engine.MaterialInstanceDynamic))))

(event EventBeginPlay)

(event EventTick
  (params (DeltaSeconds :type Float%20%28single-precision%29))
  (if (Variables|Default|GetbIsActive)
    (Transformation|SetWorldLocation (Variables|Default|GetStaticMesh) (+ (* (Variables|Default|GetVelocity) DeltaSeconds) (Transformation|GetWorldLocation (Variables|Default|GetStaticMesh))) true false)))

(fn ConstructionScript
  (bind _staticmesh (Variables|Default|GetStaticMesh))
  (Transformation|SetWorldScale3D (Variables|Default|GetStaticMesh) (Variables|Default|GetScale))
  (bind _returnvalue (Rendering|Material|CreateDynamicMaterialInstance _staticmesh 0 (Rendering|Material|GetMaterial _staticmesh 0) "None" :!class /Script/Engine.PrimitiveComponent))
  (Variables|Default|SetDynMaterial _returnvalue))

(fn DisableNote
  (Variables|Default|SetbIsActive false)
  (Rendering|SetVisibility (Variables|Default|GetStaticMesh) false true))

(fn EnableNote
  (Variables|Default|SetbIsActive true)
  (Rendering|SetVisibility (Variables|Default|GetStaticMesh) true true))

(fn SetEmissive
  (params (NewEmissiveIntensity :type Float%20%28single-precision%29))
  (Rendering|Material|SetScalarParameterValue (Variables|Default|GetDynMaterial) "EmissiveIntensity" NewEmissiveIntensity :!class /Script/Engine.MaterialInstanceDynamic)
  (Variables|Default|SetEmissiveStreakVal NewEmissiveIntensity))