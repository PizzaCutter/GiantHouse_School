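; Manages the pill minigame, which starts once a pill box is picked up and counts collected pills with a pulsing display.
; Tick runs the countdown and spawns random-colored pills inside a box, with curves over elapsed time setting delay and amount.
; A deleter volume destroys stray pills.
; When the delay curve's time range ends, it shows thanks, unlocks info, fades out and opens the player death map.
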(event OnComponentBeginOverlap(BC_PillDeleter)
  (params (OverlappedComponent :type Primitive%20Component%20Object%20Reference) (OtherActor :type Actor%20Object%20Reference) (OtherComp :type Primitive%20Component%20Object%20Reference) (OtherBodyIndex :type Integer) (bFromSweep :type Boolean) (SweepResult :type Hit%20Result%20Structure%20%28by%20ref%29))
  (bind _asbp_interactive_pill (Utilities|Casting|CastToBP_InteractivePill OtherActor))
  (Default|DestroyPill _asbp_interactive_pill))

(event Custom|CheckGameOver
  (if (>= (Variables|Default|GetElapsedTime) (.MaxTime (Math|Curves|GetTimeRange (Variables|Default|GetSpawnDelayCurve))))
    (Variables|Default|SetIsPlaying false)
    (Rendering|SetVisibility (Variables|Default|GetTR_Thanks) true false)
    (Rendering|SetVisibility (Variables|Default|GetTR_TimerStatic) false true)
    (bind _asbp_game_instance (Utilities|Casting|CastToBP_GameInstance (Game|GetGameInstance)))
    (Variables|/Game/Blueprints/BP_GameInstance.BP_GameInstance_C|SetLevelLoadOptions _asbp_game_instance "Pill")
    (Default|UnlockInfo _asbp_game_instance "NewEnumerator3")
    (Utilities|FlowControl|Delay 5.0)
    (CameraFades|StartCameraFade (Game|GetPlayerCameraManager 0) 0.0 1.0 (Variables|/Game/Blueprints/BP_GameInstance.BP_GameInstance_C|GetFadeTime _asbp_game_instance) "(R=1.000000,G=1.000000,B=1.000000,A=1.000000)" false true)
    (Utilities|FlowControl|Delay (Variables|/Game/Blueprints/BP_GameInstance.BP_GameInstance_C|GetFadeTime _asbp_game_instance))
    (Game|OpenLevel(byName) "MAP_PlayerDeadScene")))

(event Custom|StartPulse
  (bind (_direction _emissiveintensityval _scaleval) (Timeline|PulseTimeLine PlayFromStart)
    (:Update
      (Rendering|Material|SetScalarParameterValue (Variables|Default|GetPillCounterMaterial) "None" _emissiveintensityval :!class /Script/Engine.MaterialInstanceDynamic)
      (Transformation|SetRelativeScale3D (Variables|Default|GetTR_PillCountStatic) (Math|Conversions|ToVector(Float) _scaleval)))))

(event EventBeginPlay
  (bind _tr_pillcount (Variables|Default|GetTR_PillCount))
  (bind _outactors (Actor|GetAllActorsOfClass "/Game/Blueprints/Minigames/Pill/BP_PillBox.BP_PillBox_C"))
  (Variables|Default|SetPillBoxes _outactors)
  (bind _returnvalue (Rendering|Material|CreateDynamicMaterialInstance _tr_pillcount 0 (Rendering|Material|GetMaterial _tr_pillcount 0) "None" :!class /Script/Engine.PrimitiveComponent))
  (bind _output_get (Variables|Default|SetPillCounterMaterial _returnvalue))
  (Rendering|Material|SetMaterial (Variables|Default|GetTR_PillCountStatic) 0 _output_get))

(event EventTick
  (params (DeltaSeconds :type Float%20%28single-precision%29))
  (if (Variables|Default|GetIsPlaying)
    ;[1 1 1] play tick
    (Utilities|FlowControl|Sequence
      (:then_0
        ;;[1 1 1] update timer
        (Variables|Default|SetElapsedTime (+ (Utilities|Time|GetWorldDeltaSeconds) (Variables|Default|GetElapsedTime))))
      (:then_1
        ;;[1 1 1] update the text
        (CallFunction|UpdateText))
      (:then_2
        ;;[1 1 1] spawn pill at random intervals
        (Utilities|FlowControl|Delay (Math|Curves|GetFloatValue (Variables|Default|GetSpawnDelayCurve) (Utilities|GetClampedElapsedTime)))
        (if (Variables|Default|GetIsPlaying)
          (CallFunction|SpawnPill)))
      (:then_3
        (CallFunction|CheckGameOver)))
    (else
      (CallFunction|CheckStartPlaying))))

(fn ConstructionScript
  (Utilities|FlowControl|Sequence
    (:then_0
      (bind _returnvalue (Rendering|Material|CreateDynamicMaterialInstance "/Game/Materials/Pill/M_PillGreen.M_PillGreen" "None" :!class /Script/Engine.KismetMaterialLibrary))
      (Utilities|Array|Add (Variables|Default|GetPillMaterials) _returnvalue))
    (:then_1
      (bind _returnvalue_2 (Rendering|Material|CreateDynamicMaterialInstance "/Game/Materials/Pill/M_PillBlue.M_PillBlue" "None" :!class /Script/Engine.KismetMaterialLibrary))
      (Utilities|Array|Add (Variables|Default|GetPillMaterials) _returnvalue_2))
    (:then_2
      (bind _returnvalue_3 (Rendering|Material|CreateDynamicMaterialInstance "/Game/Materials/Pill/M_PillRed.M_PillRed" "None" :!class /Script/Engine.KismetMaterialLibrary))
      (Utilities|Array|Add (Variables|Default|GetPillMaterials) _returnvalue_3))
    (:then_3
      (bind _returnvalue_4 (Rendering|Material|CreateDynamicMaterialInstance "/Game/Materials/Pill/M_PillYellow.M_PillYellow" "None" :!class /Script/Engine.KismetMaterialLibrary))
      (Utilities|Array|Add (Variables|Default|GetPillMaterials) _returnvalue_4))
    (:then_4
      (Rendering|SetVisibility (Variables|Default|GetTR_Thanks) false false)
      (Rendering|SetVisibility (Variables|Default|GetTR_TimerStatic) false true)
      (Rendering|SetVisibility (Variables|Default|GetTR_PillCountStatic) false true))))

(fn SpawnPill
  (for _index (range 1 (Math|Float|Truncate (Math|Curves|GetFloatValue (Variables|Default|GetSpawnAmountCurve) (Variables|Default|GetElapsedTime))))
    (LocalVariables|SetRandomLocation (Utilities|GetRandomSpawnLocation))
    (switch int (Math|Random|RandomIntegerinRange 0 3)
      (:0
        (Game|SpawnActorfromClass "/Game/Blueprints/Minigames/Pill/BP_InteractivePill.BP_InteractivePill_C" (Math|Transform|MakeTransform (LocalVariables|GetRandomLocation) "0, 0, 0" "1,1,1") "AlwaysSpawn" 0 "NewEnumerator0" (Utilities|Array|Get(acopy) (Variables|Default|GetPillMaterials)) 0))
      (:1
        (Game|SpawnActorfromClass "/Game/Blueprints/Minigames/Pill/BP_InteractivePill.BP_InteractivePill_C" (Math|Transform|MakeTransform (LocalVariables|GetRandomLocation) "0, 0, 0" "1,1,1") "AlwaysSpawn" 0 "NewEnumerator1" (Utilities|Array|Get(acopy) (Variables|Default|GetPillMaterials) 1) 0))
      (:2
        (Game|SpawnActorfromClass "/Game/Blueprints/Minigames/Pill/BP_InteractivePill.BP_InteractivePill_C" (Math|Transform|MakeTransform (LocalVariables|GetRandomLocation) "0, 0, 0" "1,1,1") "AlwaysSpawn" 0 "NewEnumerator2" (Utilities|Array|Get(acopy) (Variables|Default|GetPillMaterials) 2) 0))
      (:3
        (Game|SpawnActorfromClass "/Game/Blueprints/Minigames/Pill/BP_InteractivePill.BP_InteractivePill_C" (Math|Transform|MakeTransform (LocalVariables|GetRandomLocation) "0, 0, 0" "1,1,1") "AlwaysSpawn" 0 "NewEnumerator3" (Utilities|Array|Get(acopy) (Variables|Default|GetPillMaterials) 3) 0)))
    (Utilities|FlowControl|Sequence
      (:then_0
        (Audio|PlaySoundatLocation "/Game/Audio/SFX/SFX_PillSpawn_Cue.SFX_PillSpawn_Cue" (LocalVariables|GetRandomLocation) "0, 0, 0" 0.01 (Math|Random|RandomFloatinRange 0.8 1.2) 0.0 0 0 0)))))

(fn CheckStartPlaying
  (if (not (Variables|Default|GetIsPlaying))
    (for _array_element (Variables|Default|GetPillBoxes)
      (Utilities|IsValid _array_element
        (:Is%20Valid
          (if (Variables|/Game/Blueprints/Minigames/Pill/BP_PillBox.BP_PillBox_C|GetbIsPickedUp _array_element)
            (Math|Integer|IncrementInt (LocalVariables|GetCounter))))))
    (if (>= (LocalVariables|GetCounter) 1)
      (CallFunction|StartPlaying))))

(fn StartPlaying
  (Variables|Default|SetIsPlaying true)
  (Variables|Default|SetPillsCollected 0)
  (CallFunction|SpawnPill)
  (Rendering|SetVisibility (Variables|Default|GetTR_TimerStatic) true true)
  (Rendering|SetVisibility (Variables|Default|GetTR_PillCountStatic) true true)
  (Rendering|SetVisibility (Variables|Default|GetTR_GameInfo) false false))

(fn PillCollected
  (bind _result (Math|Integer|IncrementInt (Variables|Default|GetPillsCollected))
    (:%20%20
      (Rendering|Components|TextRender|SetText (Variables|Default|GetTR_PillCount) (Utilities|Text|ToText(Integer) _result))
      (CallFunction|StartPulse)
      (Development|PrintString "PILL COLLECTED"))))

(fn UpdateText
  (Rendering|Components|TextRender|SetText (Variables|Default|GetTR_Timer) (Utilities|Text|ToText(Integer) (Math|Float|Floor (- (.MaxTime (Math|Curves|GetTimeRange (Variables|Default|GetSpawnDelayCurve))) (Utilities|GetClampedElapsedTime))))))