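; Pill box trigger that warps the player into the pill minigame, unless the game instance marks that minigame done.
; When either of the pawn's hand spheres overlaps the box and the player is not already dying, it sets dying, saves the pawn location and shows a spring-text warning.
; After a delay it fades the camera to white and opens the M_PillGame level.
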(event OnComponentBeginOverlap(Box)
  (params (OverlappedComponent :type Primitive%20Component%20Object%20Reference) (OtherActor :type Actor%20Object%20Reference) (OtherComp :type Primitive%20Component%20Object%20Reference) (OtherBodyIndex :type Integer) (bFromSweep :type Boolean) (SweepResult :type Hit%20Result%20Structure%20%28by%20ref%29))
  (bind _asbp_game_instance (Utilities|Casting|CastToBP_GameInstance (Game|GetGameInstance)))
  (if (not (Variables|/Game/Blueprints/BP_GameInstance.BP_GameInstance_C|GetbPillGameDone _asbp_game_instance))
    (bind _asbp_base_pawn (Utilities|Casting|CastToBP_BasePawn OtherActor))
    ;[1 1 1] CHEKC IF THE HAND SPHERES ARE VALID
    (Utilities|IsValid (Variables|/Script/GiantHouseDEV.BasePawn|GetpHandSphereL _asbp_base_pawn)
      (:Is%20Valid
        (Utilities|IsValid (Variables|/Script/GiantHouseDEV.BasePawn|GetpHandSphereR _asbp_base_pawn)
          (:Is%20Valid
            ;[1 1 1] CHECK IF THE OVERLAP IS WITH ONE OF THE HANDS
            (if (or (== (Variables|/Script/GiantHouseDEV.BasePawn|GetpHandSphereL _asbp_base_pawn) OtherComp) (== (Variables|/Script/GiantHouseDEV.BasePawn|GetpHandSphereR _asbp_base_pawn) OtherComp))
              ;[1 1 1] CHECK IF THE PLAYER IS DYING IF NOT WE KILL HIM
              (if (not (Class|BasePawn|IsDying (Variables|/Game/Blueprints/BP_GameInstance.BP_GameInstance_C|GetBasePawn _asbp_game_instance)))
                (bind _asbp_game_instance_2 (Utilities|Casting|CastToBP_GameInstance (Game|GetGameInstance)))
                (Class|BasePawn|SetDying (Variables|/Game/Blueprints/BP_GameInstance.BP_GameInstance_C|GetBasePawn _asbp_game_instance_2) true)
                ;[1 1 1] save the pawn location so we can be warped back here
                (bind _asbp_game_instance_3 (Utilities|Casting|CastToBP_GameInstance (Game|GetGameInstance)))
                (Default|SavePawnLocation _asbp_game_instance_3)
                ;[1 1 1] Show the player what happened
                (Default|SetSpringText (Variables|/Game/Blueprints/BP_GameInstance.BP_GameInstance_C|GetBasePawn _asbp_game_instance_3) "YOU TOUCHED THE PILL BOX 
YOU ARE BEING WARPED TO A MINIGAME" 0.5)
                (Default|DisableOverrideSpringText (Variables|/Game/Blueprints/BP_GameInstance.BP_GameInstance_C|GetBasePawn _asbp_game_instance_3))
                (Utilities|FlowControl|Delay 5.0)
                ;[1 1 1] SAVE SPAWN LOCATION | CAMERA FADE | TRANSITION TO DIFFERENT LEVEL
                (bind _asbp_game_instance_4 (Utilities|Casting|CastToBP_GameInstance (Game|GetGameInstance)))
                (CameraFades|StartCameraFade (Game|GetPlayerCameraManager 0) 0.0 1.0 (Variables|/Game/Blueprints/BP_GameInstance.BP_GameInstance_C|GetFadeTime _asbp_game_instance_4) "(R=1.000000,G=1.000000,B=1.000000,A=1.000000)" false true)
                (Utilities|FlowControl|Delay (Variables|/Game/Blueprints/BP_GameInstance.BP_GameInstance_C|GetFadeTime _asbp_game_instance_4))
                (Game|OpenLevel(byName) "M_PillGame")))))))))

(fn ConstructionScript)