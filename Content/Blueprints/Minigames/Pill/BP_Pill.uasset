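; BP_Pill is a pill actor for the Pill minigame that starts with randomized motion and spin.
; On BeginPlay it adds a random direction to its Velocity, rescales it to PillSpeed, and stores a random RotationVelocity scaled by RotationSpeed.
; It also adds random angular velocity to the static mesh through physics, then applies its Material variable to the first slot.
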(event EventBeginPlay
  (Utilities|FlowControl|Sequence
    (:then_0
      (Variables|Default|SetVelocity (* (Math|Vector|Normalize (+ (Variables|Default|GetVelocity) (Math|Random|RandomUnitVector))) (Variables|Default|GetPillSpeed)))
      (Variables|Default|SetRotationVelocity (* (Math|Random|RandomRotator true) (Variables|Default|GetRotationSpeed)))
      (Class|PrimitiveComponent|SetPhysicsAngularVelocityinDegrees (Variables|Default|GetStaticMesh) (* (Math|Random|RandomUnitVector) (Variables|Default|GetRotationSpeed)) true "None"))
    (:then_1
      (Rendering|Material|SetMaterial (Variables|Default|GetStaticMesh) 0 (Variables|Default|GetMaterial)))))

(fn ConstructionScript)