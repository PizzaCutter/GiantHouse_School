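; Hazard spawner for the climbing minigame that, while active, tracks the player's collider in X and Y at its own height.
; A latent Delay inside Tick paces the spawning of BP_Hazard actors at a random Y offset, passing on speed and rotation speed.
; ReduceDelay shortens that delay by a fixed step at timed intervals, so hazards come more frequently over time, with no lower limit.
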(event EventBeginPlay)

(event Collision|EventActorBeginOverlap
  (params (OtherActor :type Actor%20Object%20Reference)))

(event EventTick
  (params (DeltaSeconds :type Float%20%28single-precision%29))
  (bind _returnvalue (Transformation|GetActorTransform))
  (bind _player (Variables|Default|GetPlayer))
  (bind _randomrange (Variables|Default|GetRandomRange))
  (bind (_location _rotation _scale) (Math|Transform|BreakTransform _returnvalue))
  (bind _pcameracollider (Variables|/Script/GiantHouseDEV.BasePawn|GetpCameraCollider _player))
  (bind (_x _y _z) (Math|Vector|BreakVector _location))
  (bind _returnvalue_2 (Transformation|GetWorldLocation _pcameracollider))
  (bind (_x_2 _y_2) (Math|Vector|BreakVector _returnvalue_2))
  (if (Variables|Default|GetbIsActive)
    (Variables|Default|SetTimer (+ (Variables|Default|GetTimer) DeltaSeconds))
    (CallFunction|ReduceDelay)
    (Transformation|SetActorLocation (Math|Vector|MakeVector _x_2 _y_2 (.Z (Math|Vector|BreakVector (Transformation|GetActorLocation)))) false false)
    (Utilities|FlowControl|Delay (Variables|Default|GetDelayTimeToNextHazardSpawn))
    (Game|SpawnActorfromClass "/Game/Blueprints/Minigames/Climbing/BP_Hazard.BP_Hazard_C" (Math|Transform|MakeTransform (Math|Vector|MakeVector _x (+ _y (Math|Random|RandomFloatinRange (* _randomrange -1.0) _randomrange)) _z) _rotation _scale) "Undefined" 0 (Variables|Default|GetSpeed) (Variables|Default|GetRotationSpeed) 0)))

(fn ConstructionScript)

(fn ReduceDelay
  (if (<= (Variables|Default|GetTimePerDecreaseTimer) (Variables|Default|GetTimer))
    (Variables|Default|SetTimer 0.0)
    (Variables|Default|SetDelayTimeToNextHazardSpawn (- (Variables|Default|GetDelayTimeToNextHazardSpawn) (Variables|Default|GetDecreaseTimer)))
    (return)
    (else
      (return))))