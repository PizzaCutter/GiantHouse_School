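; Falling hazard for the climbing minigame that damages the player through the game manager.
; Construction reveals one of seven random household props at a random rotation and attaches the actor to the "Cliff"-tagged mesh.
; Tick moves it downward while spinning the prop.
; An outer SlowMotion overlap slows the hazard's own time and global audio pitch; hitting the pawn's camera collider triggers damage, sound and particles, then destroys it.
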(event OnComponentBeginOverlap(Damage)
  (params (OverlappedComponent :type Primitive%20Component%20Object%20Reference) (OtherActor :type Actor%20Object%20Reference) (OtherComp :type Primitive%20Component%20Object%20Reference) (OtherBodyIndex :type Integer) (bFromSweep :type Boolean) (SweepResult :type Hit%20Result%20Structure%20%28by%20ref%29))
  (bind _emmiterspawn (Variables|Default|GetEmmiterSpawn))
  (bind _returnvalue (Transformation|GetWorldTransform _emmiterspawn))
  (bind (_location _rotation _scale) (Math|Transform|BreakTransform _returnvalue))
  (bind _asbp_base_pawn (Utilities|Casting|CastToBP_BasePawn OtherActor))
  (if (== OtherComp (Variables|/Script/GiantHouseDEV.BasePawn|GetpCameraCollider _asbp_base_pawn))
    (Default|TakeDamage (Variables|Default|GetGameManager))
    (Audio|PlaySound2D "/Game/Audio/SFX/SFX_Hit_Climbing.SFX_Hit_Climbing" 1.0 1.0 0.0 0 0)
    (Effects|SpawnEmitteratLocation "/Game/FX/P_Groundburst.P_Groundburst" _location _rotation _scale)
    (Actor|DestroyActor)))

(event OnComponentBeginOverlap(SlowMotion)
  (params (OverlappedComponent :type Primitive%20Component%20Object%20Reference) (OtherActor :type Actor%20Object%20Reference) (OtherComp :type Primitive%20Component%20Object%20Reference) (OtherBodyIndex :type Integer) (bFromSweep :type Boolean) (SweepResult :type Hit%20Result%20Structure%20%28by%20ref%29))
  (Utilities|Casting|CastToBasePawn OtherActor)
  (Variables|Default|SetCustomTimeDilation 0.3)
  (Class|GameplayStatics|SetGlobalPitchModulation 0.3 0.5))

(event OnComponentEndOverlap(SlowMotion)
  (params (OverlappedComponent :type Primitive%20Component%20Object%20Reference) (OtherActor :type Actor%20Object%20Reference) (OtherComp :type Primitive%20Component%20Object%20Reference) (OtherBodyIndex :type Integer))
  (Utilities|Casting|CastToBasePawn OtherActor)
  (Variables|Default|SetCustomTimeDilation 1.0)
  (Class|GameplayStatics|SetGlobalPitchModulation 1.0 0.5))

(event EventBeginPlay
  (bind _outactors (Actor|GetAllActorsOfClass "/Game/Blueprints/Minigames/Climbing/BP_GameManager.BP_GameManager_C"))
  (Variables|Default|SetGameManager (Utilities|Array|Get(acopy) _outactors)))

(event Collision|EventActorBeginOverlap
  (params (OtherActor :type Actor%20Object%20Reference)))

(event EventTick
  (params (DeltaSeconds :type Float%20%28single-precision%29))
  (bind _visibleprop (Variables|Default|GetVisibleProp))
  (Transformation|AddActorWorldOffset (* (Math|Vector|MakeVector 0.0 0.0 -1.0) (* (Variables|Default|GetSpeed) DeltaSeconds)))
  (if (Utilities|IsValid _visibleprop)
    (Transformation|AddWorldRotation _visibleprop (Math|Rotator|MakeRotator 0.0 (* (Variables|Default|GetRotationSpeed) DeltaSeconds) 0.0) false false)))

(fn ConstructionScript
  (bind _knife (Variables|Default|GetKnife))
  (bind _bowl (Variables|Default|GetBowl))
  (bind _candlestick (Variables|Default|GetCandlestick))
  (bind _vase (Variables|Default|GetVase))
  (bind _pepper (Variables|Default|GetPepper))
  (bind _salt (Variables|Default|GetSalt))
  (bind _mug (Variables|Default|GetMug))
  (switch int (Math|Random|RandomInteger 7)
    (:0
      (Development|SetHiddeninGame _knife false false)
      (bind _output_get (Variables|Default|SetVisibleProp _knife)))
    (:1
      (Development|SetHiddeninGame _bowl false false)
      (bind _output_get_2 (Variables|Default|SetVisibleProp _bowl)))
    (:2
      (Development|SetHiddeninGame _candlestick false false)
      (bind _output_get_3 (Variables|Default|SetVisibleProp _candlestick)))
    (:3
      (Development|SetHiddeninGame _vase false false)
      (bind _output_get_4 (Variables|Default|SetVisibleProp _vase)))
    (:4
      (Development|SetHiddeninGame _mug false false)
      (bind _output_get_5 (Variables|Default|SetVisibleProp _mug)))
    (:5
      (Development|SetHiddeninGame _salt false false)
      (bind _output_get_6 (Variables|Default|SetVisibleProp _salt)))
    (:6
      (Development|SetHiddeninGame _pepper false false)
      (bind _output_get_7 (Variables|Default|SetVisibleProp _pepper))))
  (Transformation|SetWorldRotation _output_get_2 (Math|Random|RandomRotator false) false false)
  (bind _outactors (Actor|GetAllActorswithTag "Cliff"))
  (bind _asstatic_mesh_actor (Utilities|Casting|CastToStaticMeshActor (Utilities|Array|Get(acopy) _outactors)))
  (bind _output_get_8 (Variables|Default|SetCliff _asstatic_mesh_actor))
  (Transformation|AttachActorToActor _output_get_8 "None" "KeepWorld" "KeepWorld" "KeepWorld" false))