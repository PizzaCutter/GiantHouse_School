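; Game manager for the climbing minigame that plays ambient sound, sets the player's starting rotation and tracks lives.
; A box overlap recycles static mesh pieces for endless climbing, teleporting the lowest sibling under the shared attach parent above the highest.
; TakeDamage decrements lives, and Tick watches for zero to fade the camera, unlock info on the game instance and open the death scene map.
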(event OnComponentBeginOverlap(Box)
  (params (OverlappedComponent :type Primitive%20Component%20Object%20Reference) (OtherActor :type Actor%20Object%20Reference) (OtherComp :type Primitive%20Component%20Object%20Reference) (OtherBodyIndex :type Integer) (bFromSweep :type Boolean) (SweepResult :type Hit%20Result%20Structure%20%28by%20ref%29))
  (bind _asstatic_mesh_actor (Utilities|Casting|CastToStaticMeshActor OtherActor))
  (bind (__lowest __highest) (CallFunction|FindLowestandHighestIdx (Actor|GetAttachedActors (Actor|GetAttachParentActor _asstatic_mesh_actor))))
  (Transformation|SetActorLocation (Utilities|Array|Get(acopy) (Actor|GetAttachedActors (Actor|GetAttachParentActor _asstatic_mesh_actor)) __lowest) (+ (Transformation|GetActorLocation (Utilities|Array|Get(acopy) (Actor|GetAttachedActors (Actor|GetAttachParentActor _asstatic_mesh_actor)) __highest)) "0, 0,400.000000") false true))

(event EventBeginPlay
  (Audio|PlaySoundatLocation "/Game/Audio/AMB/AMB_ClimbingNoise_Cue.AMB_ClimbingNoise_Cue" (Transformation|GetActorLocation) "0, 0, 0" 1.0 1.0 0.0 0 0 0))

(event Collision|EventActorBeginOverlap
  (params (OtherActor :type Actor%20Object%20Reference)))

(event EventTick
  (params (DeltaSeconds :type Float%20%28single-precision%29))
  (if (<= (Variables|Default|GetLives) 0)
    (CameraFades|StartCameraFade :self (Game|GetPlayerCameraManager 0) :ToAlpha 1.0 :Duration 0.5)
    (bind _asbp_game_instance (Utilities|Casting|CastToBP_GameInstance (Game|GetGameInstance)))
    (Default|UnlockInfo _asbp_game_instance "NewEnumerator1")
    (Variables|/Game/Blueprints/BP_GameInstance.BP_GameInstance_C|SetLevelLoadOptions _asbp_game_instance "Climbing")
    (Utilities|FlowControl|Delay 0.5)
    (Game|OpenLevel(byName) "MAP_PlayerDeadScene" true "Climbing")
    (else
      (Utilities|FlowControl|DoOnce false
        (:Completed
          (bind _asbp_game_instance_2 (Utilities|Casting|CastToBP_GameInstance (Game|GetGameInstance)))
          (Pawn|SetControlRotation (Pawn|GetController (Variables|/Game/Blueprints/BP_GameInstance.BP_GameInstance_C|GetBasePawn _asbp_game_instance_2)) (Variables|Default|GetPawnRotation)))))))

(fn ConstructionScript)

(fn TakeDamage
  (Math|Integer|DecrementInt (Variables|Default|GetLives)))

(fn FindLowestandHighestIdx
  (params (Actors :type Array%20of%20Actor%20Object%20References))
  (for (_array_element _array_index) Actors
    (if (<= (LocalVariables|Gethighest) (.Z (Math|Vector|BreakVector (Transformation|GetActorLocation _array_element))))
      (LocalVariables|Sethighest (.Z (Math|Vector|BreakVector (Transformation|GetActorLocation _array_element))))
      (LocalVariables|SetidxOfHighest _array_index))
    (if (<= (.Z (Math|Vector|BreakVector (Transformation|GetActorLocation _array_element))) (LocalVariables|Getlowest))
      (LocalVariables|Setlowest (.Z (Math|Vector|BreakVector (Transformation|GetActorLocation _array_element))))
      (LocalVariables|SetidxOfLowest _array_index)))
  (return (LocalVariables|GetidxOfLowest) (LocalVariables|GetidxOfHighest)))