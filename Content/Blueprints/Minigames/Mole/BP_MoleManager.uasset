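; Manager for the whack-a-mole minigame: runs the round, timer, score and music.
; All moles show at setup, and the first hit starts play, where Tick pops random available moles with curve-driven delays and idle times.
; Floating score texts overlapping a volume add curve-scaled points with a scrambled-number glow animation.
; Elapsed time drives timer pulses and the pawn's hand burn, until time-up unlocks info, fades out and opens the player-dead map.
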(event OnComponentBeginOverlap(BCC_DeleteVolume)
  (params (OverlappedComponent :type Primitive%20Component%20Object%20Reference) (OtherActor :type Actor%20Object%20Reference) (OtherComp :type Primitive%20Component%20Object%20Reference) (OtherBodyIndex :type Integer) (bFromSweep :type Boolean) (SweepResult :type Hit%20Result%20Structure%20%28by%20ref%29))
  (bind _asbp_floating_text_renderer (Utilities|Casting|CastToBP_FloatingTextRenderer OtherActor))
  (ScoreSystem|AddScore (Variables|/Game/Blueprints/Minigames/Mole/BP_FloatingTextRenderer.BP_FloatingTextRenderer_C|GetScore _asbp_floating_text_renderer))
  (Actor|DestroyActor _asbp_floating_text_renderer)
  (bind _emissiveboost (Timeline|AddScoreAnimation PlayFromStart)
    (:Update
      ;[1 1 1] RANDOM NUMBER + EMISSIVE ANIMATION
      (Text|RandomTextScore)
      (Rendering|Material|SetScalarParameterValue (Variables|Default|GetScoreTextDynMaterial) "EmissiveIntensity" _emissiveboost :!class /Script/Engine.MaterialInstanceDynamic))
    (:Finished
      (Text|UpdateTextScore))))

(event OnComponentBeginOverlap(BCC_IncreaseBrightnessVolume)
  (params (OverlappedComponent :type Primitive%20Component%20Object%20Reference) (OtherActor :type Actor%20Object%20Reference) (OtherComp :type Primitive%20Component%20Object%20Reference) (OtherBodyIndex :type Integer) (bFromSweep :type Boolean) (SweepResult :type Hit%20Result%20Structure%20%28by%20ref%29))
  (bind _asbp_floating_text_renderer (Utilities|Casting|CastToBP_FloatingTextRenderer OtherActor))
  (Default|BoostEmissive _asbp_floating_text_renderer))

(event Custom|AnyMoleHit
  (if (not (Variables|Default|GetIsPlaying))
    (MoleSystem|HideAllMoles)
    (Utilities|FlowControl|Delay 3.0)
    (Variables|Default|SetIsPlaying true)
    (Rendering|SetVisibility (Variables|Default|GetBP_SpriteMoleTutorial) false true)
    (Rendering|SetVisibility (Variables|Default|GetTRC_ScoreText) true true)
    (Rendering|SetVisibility (Variables|Default|GetTRC_Score) true true)
    (Rendering|SetVisibility (Variables|Default|GetTRC_Time) true true)
    (Audio|PlaySound2D "/Game/Audio/AMB/AMB_WhackAMoleMusic.AMB_WhackAMoleMusic" 0.1 1.0 0.0 0 0)))

(event Custom|PulseTimerText
  (Utilities|FlowControl|Delay 1.0)
  (Audio|PlaySound2D "/Game/Audio/SFX/SFX_Pulse_01.SFX_Pulse_01" 0.1 (Math|Random|RandomFloatinRange (Variables|Default|GetScoreAddMinPitch) (Variables|Default|GetScoreAddMaxPitch)) 0.0 0 0)
  (bind (_direction _emissiveboost _scale _textcolor) (Timeline|TimerTextPulse PlayFromStart)
    (:Update
      (Utilities|FlowControl|Sequence
        (:then_0
          (Rendering|Material|SetScalarParameterValue (Variables|Default|GetTimeTextDynMaterial) "EmissiveIntensity" _emissiveboost :!class /Script/Engine.MaterialInstanceDynamic))
        (:then_1
          (Transformation|SetRelativeScale3D (Variables|Default|GetTRC_Time) (Math|Conversions|ToVector(Float) _scale)))
        (:then_2
          (Rendering|Components|TextRender|SetTextRenderColor (Variables|Default|GetTRC_Time) (Math|Conversions|ToColor(LinearColor) _textcolor)))))))

(event Custom|CompletedGame
  (Utilities|FlowControl|Sequence
    (:then_0
      (bind _asbp_base_pawn (Utilities|Casting|CastToBP_BasePawn (Pawn|GetControlledPawn (Game|GetPlayerController 0))))
      (Default|SetSpringText _asbp_base_pawn "YOU BURNED YOUR HANDS 
YOU WILL BE TELEPORTED" 0.5))
    (:then_1
      (Rendering|SetVisibility (Variables|Default|GetTRC_Time) false false))))

(event EventBeginPlay
  (Utilities|FlowControl|Sequence
    (:then_0
      (Utilities|FlowControl|Delay 0.0)
      ;[1 1 1] GET REFERENCES TO MOLES AND LET THEM JUMP UP
      (bind _outactors (Actor|GetAllActorsOfClass "/Game/Blueprints/Minigames/Mole/BP_Mole.BP_Mole_C"))
      (bind _output_get (Variables|Default|SetMoles _outactors))
      (for _array_element _output_get
        (Variables|/Game/Blueprints/Minigames/Mole/BP_Mole.BP_Mole_C|SetManager _array_element self)
        (CallFunction|SetupGame)))
    (:then_1
      (Audio|PlaySound2D "/Game/Audio/SFX/SFX_BGSound_Swamp_C.SFX_BGSound_Swamp_C" 0.05 1.0 0.0 0 0))))

(event EventTick
  (params (DeltaSeconds :type Float%20%28single-precision%29))
  (bind _clampedacumtime (Utilities|GetClampedAcumTime))
  (bind _clampedacumtime_2 (Utilities|GetClampedAcumTime))
  (bind _molepopupcurve (Variables|Default|GetMolePopUpCurve))
  (bind _moleidletimecurve (Variables|Default|GetMoleIdleTimeCurve))
  (bind _returnvalue (Math|Curves|GetVectorValue _moleidletimecurve _clampedacumtime))
  (bind _returnvalue_2 (Math|Curves|GetVectorValue _molepopupcurve _clampedacumtime_2))
  (if (Variables|Default|GetIsPlaying)
    ;[1 1 1] MAKE MOLES JUMP AND SET AN IDLE TIME
    (Utilities|FlowControl|Sequence
      (:then_0
        ;;[1 1 1] UPDATE TOTAL TIME
        (bind _output_get (Variables|Default|SetAccumulatedTime (+ (Utilities|Time|GetWorldDeltaSeconds) (Variables|Default|GetAccumulatedTime))))
        (if (<= _output_get (Variables|Default|GetGameTime))
          (Text|UpdateTextTimer)
          (Utilities|FlowControl|Delay (Math|Random|RandomFloatinRange (.x _returnvalue_2) (.y _returnvalue_2)))
          (bind _availablemole (MoleSystem|GetRandomAvailableMole))
          (Utilities|IsValid _availablemole
            (:Is%20Valid
              (Variables|/Game/Blueprints/Minigames/Mole/BP_Mole.BP_Mole_C|SetIdleTime _availablemole (Math|Random|RandomFloatinRange (.x _returnvalue) (.y _returnvalue)))
              (Default|Jump _availablemole)))
          (else
            (Utilities|FlowControl|DoOnce false
              (:Completed
                (CallFunction|CompletedGame)
                (Utilities|FlowControl|Delay 5.0)
                (CameraFades|StartCameraFade :self (Game|GetPlayerCameraManager 0) :ToAlpha 1.0 :Duration 1.0)
                (Utilities|FlowControl|Delay 1.0)
                (bind _asbp_game_instance (Utilities|Casting|CastToBP_GameInstance (Game|GetGameInstance)))
                (Default|UnlockInfo _asbp_game_instance "NewEnumerator0")
                (Variables|/Game/Blueprints/BP_GameInstance.BP_GameInstance_C|SetLevelLoadOptions _asbp_game_instance "Mole")
                (Game|OpenLevel(byName) "MAP_PlayerDeadScene" true "Mole"))))))
      (:then_1
        (if (>= (Variables|Default|GetAccumulatedTime) 55.0)
          (Utilities|FlowControl|Sequence
            (:then_0
              (Utilities|FlowControl|Gate false :!label _label
                (:Exit
                  (Audio|PlaySound2D "/Game/Audio/SFX/SFX_TimeUpLoop.SFX_TimeUpLoop" 0.05 1.0 0.0 0 0))))
            (:then_1
              (goto _label Close)))))
      (:then_2
        (bind _asbp_base_pawn (Utilities|Casting|CastToBP_BasePawn (Pawn|GetControlledPawn (Game|GetPlayerController 0))))
        (Default|LerpBurn _asbp_base_pawn (/ (Variables|Default|GetAccumulatedTime) (Variables|Default|GetGameTime)))))))

(fn ConstructionScript
  (bind _trc_score (Variables|Default|GetTRC_Score))
  (bind _trc_time (Variables|Default|GetTRC_Time))
  (Utilities|FlowControl|Sequence
    (:then_0
      ;[1 1 1] CREATE AND CACHED DYNAMIC MATERIAL FOR TIME TEXT
      (bind _returnvalue (Rendering|Material|CreateDynamicMaterialInstance _trc_time 0 (Rendering|Material|GetMaterial _trc_time 0) "None" :!class /Script/Engine.PrimitiveComponent))
      (Variables|Default|SetTimeTextDynMaterial _returnvalue))
    (:then_1
      ;[1 1 1] CREATE AND CACHED DYNAMIC MATERIAL FOR SCORE TEXT
      (bind _returnvalue_2 (Rendering|Material|CreateDynamicMaterialInstance _trc_score 0 (Rendering|Material|GetMaterial _trc_score 0) "None" :!class /Script/Engine.PrimitiveComponent))
      (Variables|Default|SetScoreTextDynMaterial _returnvalue_2))))

(fn GetRandomAvailableMole
  (bind (_moleavailable _availablemoles) (MoleSystem|MoleAvailable))
  (if _moleavailable
    (return (Utilities|Array|Get(acopy) _availablemoles (Math|Random|RandomInteger (Utilities|Array|Length _availablemoles))))
    (else
      (return 0))))

(fn MoleAvailable
  (bind _l_availablemoles (LocalVariables|GetL_AvailableMoles))
  (Utilities|Array|Clear (LocalVariables|GetL_AvailableMoles))
  (for _array_element (Variables|Default|GetMoles)
    (if (Default|CanJump _array_element)
      (Utilities|Array|Add (LocalVariables|GetL_AvailableMoles) _array_element)))
  (return (> (Utilities|Array|Length _l_availablemoles) 0) _l_availablemoles))

(fn HideAllMoles
  (for _array_element (Variables|Default|GetMoles)
    (Default|Hide _array_element)))

(fn UpdateTextTimer
  (Utilities|FlowControl|Sequence
    (:then_0
      (Rendering|Components|TextRender|SetText (Variables|Default|GetTRC_Time) (Utilities|Text|ToText(String) (Utilities|String|Append "TIME:" (Utilities|String|ToString(Integer) (- (Math|Float|Truncate (Variables|Default|GetGameTime)) (Math|Float|Truncate (Variables|Default|GetAccumulatedTime))))))))
    (:then_1
      (if (== (Math|Integer|%(Integer) (+ (Math|Float|Truncate (Variables|Default|GetAccumulatedTime)) 1) (Variables|Default|GetPulseInterval)) 0)
        (CallFunction|PulseTimerText)))))

(fn ShowAllMoles
  (for _array_element (Variables|Default|GetMoles)
    (Default|Jump _array_element)))

(fn SetupGame
  (MoleSystem|ShowAllMoles)
  (Variables|Default|SetIsPlaying false)
  (Variables|Default|SetAccumulatedTime 0.0)
  (Variables|Default|SetTotalScore 0)
  (Text|UpdateTextTimer)
  (Text|UpdateTextScore)
  (Rendering|SetVisibility (Variables|Default|GetBP_SpriteMoleTutorial) true true)
  (Rendering|SetVisibility (Variables|Default|GetTRC_ScoreText) false true)
  (Rendering|SetVisibility (Variables|Default|GetTRC_Score) false true)
  (Rendering|SetVisibility (Variables|Default|GetTRC_Time) false true))

(fn AddScore
  (params (AddedScore :type Integer))
  (if (Variables|Default|GetIsPlaying)
    (Variables|Default|SetTotalScore (+ (Variables|Default|GetTotalScore) (Math|Float|Truncate (* AddedScore (.z (Math|Curves|GetVectorValue (Variables|Default|GetMolePopUpCurve) (Variables|Default|GetAccumulatedTime)))))))
    (Text|UpdateTextScore)
    (return (Variables|Default|GetTotalScore))))

(fn UpdateTextScore
  (Rendering|Components|TextRender|SetText (Variables|Default|GetTRC_Score) (Utilities|Text|ToText(String) (Utilities|String|ToString(Integer) (Variables|Default|GetTotalScore)))))

(fn GetFloatingTextTarget
  (bind _trc_score (Variables|Default|GetTRC_Score))
  (bind _returnvalue (Class|TextRenderComponent|GetTextWorldSize _trc_score))
  (return (+ (Transformation|GetWorldLocation _trc_score) (Math|Vector|MakeVector (/ (.x _returnvalue) 2.0) (/ (.y _returnvalue) 2.0) 0.0))))

(fn RandomTextScore
  (Rendering|Components|TextRender|SetText (Variables|Default|GetTRC_Score) (Utilities|Text|ToText(String) (Utilities|String|ToString(Integer) (Math|Random|RandomInteger (+ 1 (Variables|Default|GetTotalScore)))))))