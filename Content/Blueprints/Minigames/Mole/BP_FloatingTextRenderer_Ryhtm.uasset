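; Floating text actor for the Mole rhythm minigame that shows a hit quality rating as MISS, BAD, GOOD or PERFECT.
; On BeginPlay it sets the rating text, picks a random color from its list and applies an emissive intensity to a dynamic material created in the construction script.
; Tick moves it along a direction at a set velocity until it destroys itself after a short delay.
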(event EventBeginPlay
  (bind _colors (Variables|Default|GetColors))
  (bind _returnvalue (Utilities|Array|Length _colors))
  (Utilities|FlowControl|Sequence
    (:then_0
      ;[1 1 1] GET A RANDOM COLOR FOR THE TEXT
      (if (> _returnvalue 0)
        (Rendering|Components|TextRender|SetTextRenderColor (Variables|Default|GetTextRender) (Math|Conversions|ToColor(LinearColor) (Utilities|Array|Get(acopy) (Variables|Default|GetColors) (Math|Random|RandomInteger _returnvalue))))))
    (:then_1
      (switch Utilities|FlowControl|Switch|SwitchoneHITQUALITY (Variables|Default|GetHitQuality)
        (:NewEnumerator3
          (Variables|Default|SetHitQualityText "MISS"))
        (:NewEnumerator0
          (Variables|Default|SetHitQualityText "BAD"))
        (:NewEnumerator1
          (Variables|Default|SetHitQualityText "GOOD"))
        (:NewEnumerator2
          (Variables|Default|SetHitQualityText "PERFECT"))))
    (:then_2
      (Rendering|Components|TextRender|SetText (Variables|Default|GetTextRender) (Variables|Default|GetHitQualityText)))
    (:then_3
      (Rendering|Material|SetScalarParameterValue (Variables|Default|GetTextMaterial) "EmissiveIntensity" (Variables|EmissiveBoost|GetEmissiveIntensity) :!class /Script/Engine.MaterialInstanceDynamic))
    (:then_4
      (Utilities|FlowControl|Delay 2.0)
      (Actor|DestroyActor))))

(event EventTick
  (params (DeltaSeconds :type Float%20%28single-precision%29))
  ;[1 1 1] MOVE THE TEXT
  (Transformation|SetActorLocation (+ (Transformation|GetActorLocation) (* (* (Variables|Movement|GetDirection) (Variables|Movement|GetVelocity)) (Utilities|Time|GetWorldDeltaSeconds))) false true))

(fn ConstructionScript
  (bind _textrender (Variables|Default|GetTextRender))
  (bind _returnvalue (Rendering|Material|CreateDynamicMaterialInstance _textrender 0 (Rendering|Material|GetMaterial _textrender 0) "None" :!class /Script/Engine.PrimitiveComponent))
  (Variables|Default|SetTextMaterial _returnvalue))