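; Whack-a-mole minigame actor that pops up, hides after a delay and can be hit by the VR player.
; Its state lives in the animation Blueprint, read and written through helper functions that gate jumping, hiding and hitting.
; A hit registers when a pawn component's vertical speed between box overlap begin and end reaches a force threshold.
; Hits notify the Manager, play sounds and haptics, and spawn floating score text during play.
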(event OnComponentBeginOverlap(Box)
  (params (OverlappedComponent :type Primitive%20Component%20Object%20Reference) (OtherActor :type Actor%20Object%20Reference) (OtherComp :type Primitive%20Component%20Object%20Reference) (OtherBodyIndex :type Integer) (bFromSweep :type Boolean) (SweepResult :type Hit%20Result%20Structure%20%28by%20ref%29))
  (bind _asbp_base_pawn (Utilities|Casting|CastToBP_BasePawn OtherActor))
  (if (and (!= (Variables|/Script/GiantHouseDEV.BasePawn|GetpCameraCollider _asbp_base_pawn) OtherComp) (!= OtherComp (Variables|/Game/Blueprints/Gameplay/BP_BasePawn.BP_BasePawn_C|GetBP_ObjectiveBookL _asbp_base_pawn)))
    (Variables|Default|SetCachedActorComp OtherComp)
    (Variables|Default|SetOverlapTimer 0.0)
    (Variables|Default|SetOverlapStartLocation (Transformation|GetWorldLocation OtherComp))))

(event OnComponentEndOverlap(Box)
  (params (OverlappedComponent :type Primitive%20Component%20Object%20Reference) (OtherActor :type Actor%20Object%20Reference) (OtherComp :type Primitive%20Component%20Object%20Reference) (OtherBodyIndex :type Integer))
  (bind _molestate (CallFunction|GetMoleState))
  (Utilities|Casting|CastToBP_BasePawn OtherActor)
  (if (== OtherComp (Variables|Default|GetCachedActorComp))
    (Utilities|FlowControl|Sequence
      (:then_0
        (if (>= (/ (Math|Float|Absolute(Float) (- (.z (Variables|Default|GetOverlapStartLocation)) (.z (Transformation|GetWorldLocation (Variables|Default|GetCachedActorComp))))) (Variables|Default|GetOverlapTimer)) (Variables|Default|GetForceNeeded))
          (if (or (Utilities|Enum|Equal(Enum) _molestate "NewEnumerator2") (Utilities|Enum|Equal(Enum) _molestate "NewEnumerator1"))
            (CallFunction|Hit)
            (Development|PrintString "HIT" false false "(R=0.176807,G=1.000000,B=0.000000,A=1.000000)"))))
      (:then_1
        (Variables|Default|SetCachedActorComp 0)))))

(event Custom|Jump
  (bind _manager (Variables|Default|GetManager))
  (if (CallFunction|CanJump)
    (CallFunction|SetMoleState "NewEnumerator1")
    (Audio|PlaySoundatLocation "/Game/Audio/SFX/SFX_Foomp_01_Cue.SFX_Foomp_01_Cue" (Transformation|GetActorLocation) "0, 0, 0" 0.1 (Math|Random|RandomFloatinRange (Variables|Default|GetPopUpMinPitch) (Variables|Default|GetPopUpMaxPitch)) 0.0 0 0 0)
    (Utilities|FlowControl|Sequence
      (:then_0
        (if (> (Variables|Default|GetIdleTime) 0.0)
          (Utilities|FlowControl|RetriggerableDelay (Variables|Default|GetIdleTime))
          (CallFunction|Hide)))
      (:then_1
        (Utilities|IsValid _manager
          (:Is%20Valid
            (if (Variables|/Game/Blueprints/Minigames/Mole/BP_MoleManager.BP_MoleManager_C|GetIsPlaying _manager)
              (Utilities|FlowControl|RetriggerableDelay 5.0)
              (CallFunction|SetMoleState "NewEnumerator0"))))))))

(event Custom|Hide
  (if (not (Utilities|Enum|Equal(Enum) (CallFunction|GetMoleState) "NewEnumerator3"))
    (CallFunction|SetMoleState "NewEnumerator0")))

(event Custom|Hit
  (bind _returnvalue (Game|GetPlayerController 0))
  (bind _returnvalue_2 (Transformation|GetActorLocation))
  (Class|PlayerController|PlayHapticEffect _returnvalue "/Game/Blueprints/Gameplay/HF_Standard.HF_Standard" "Left" 1.0 false)
  (Class|PlayerController|PlayHapticEffect _returnvalue "/Game/Blueprints/Gameplay/HF_Standard.HF_Standard" "Right" 1.0 false)
  (CallFunction|SetMoleState "NewEnumerator3")
  (Default|AnyMoleHit (Variables|Default|GetManager))
  (Audio|PlaySoundatLocation "/Game/Audio/SFX/SFX_Hit_01_Cue.SFX_Hit_01_Cue" _returnvalue_2 "0, 0, 0" 0.1 (Math|Random|RandomFloatinRange (Variables|Default|GetHitMinPitch) (Variables|Default|GetHitMaxPitch)) 0.0 0 0 0)
  (Audio|PlaySoundatLocation "/Game/Audio/SFX/SXF_Sizzle_Cue.SXF_Sizzle_Cue" _returnvalue_2 "0, 0, 0" 0.1 1.0 0.0 0 0 0)
  (Class|PlayerController|PlayHapticEffect (Game|GetPlayerController 0) "/Game/Blueprints/Gameplay/HF_Standard.HF_Standard" (CallFunction|GetHand) 1.0 false)
  (if (Variables|/Game/Blueprints/Minigames/Mole/BP_MoleManager.BP_MoleManager_C|GetIsPlaying (Variables|Default|GetManager))
    (Game|SpawnActorfromClass "/Game/Blueprints/Minigames/Mole/BP_FloatingTextRenderer.BP_FloatingTextRenderer_C" (Math|Transform|MakeTransform (.location (Transformation|GetWorldTransform (Variables|Default|GetArrow))) "0, 0, 0" "1,1,1") "AlwaysSpawn" 0 (Variables|Default|GetScore) 0)))

(event EventBeginPlay
  ;[1 1 1] GET ANIMATION REFERENCE
  (bind _asabp_mole (Utilities|Casting|CastToABP_Mole (Components|SkeletalMesh|GetAnimInstance (Variables|Default|GetSkeletalMesh))))
  (Variables|Default|SetMoleAnimRef _asabp_mole))

(event EventTick
  (params (DeltaSeconds :type Float%20%28single-precision%29))
  (Variables|Default|SetOverlapTimer (+ DeltaSeconds (Variables|Default|GetOverlapTimer))))

(fn ConstructionScript)

(fn SetMoleState
  (params (NewState :type eMOLESTATE%20Enum :default "NewEnumerator0"))
  (Variables|/Game/Animations/Whack_A_Mole/ABP_Mole.ABP_Mole_C|SetMoleState (Variables|Default|GetMoleAnimRef) NewState))

(fn CanJump
  (return (Utilities|Enum|Equal(Enum) (CallFunction|GetMoleState) "NewEnumerator0")))

(fn GetMoleState
  (return (Variables|/Game/Animations/Whack_A_Mole/ABP_Mole.ABP_Mole_C|GetMoleState (Variables|Default|GetMoleAnimRef))))

(fn GetHand
  (bind _asbp_base_pawn (Utilities|Casting|CastToBP_BasePawn (Game|Player|GetPlayerPawn 0)))
  (Utilities|FlowControl|Sequence
    (:then_0
      (if (== (Variables|Default|GetCachedActorComp) (Variables|/Script/GiantHouseDEV.BasePawn|GetpHandSphereL _asbp_base_pawn))
        (return "Left")))
    (:then_1
      (if (== (Variables|Default|GetCachedActorComp) (Variables|/Script/GiantHouseDEV.BasePawn|GetpHandSphereR _asbp_base_pawn))
        (return "Right")))
    (:then_2
      (return "Special_11"))))