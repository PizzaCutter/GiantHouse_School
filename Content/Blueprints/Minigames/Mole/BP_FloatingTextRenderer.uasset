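; Floating text actor for the Mole minigame that flies toward a target supplied by BP_MoleManager.
; BeginPlay picks a random speed and color and fixes the travel direction, then Tick moves the text along it.
; A dynamic material instance drives emissive intensity from travel progress toward the target, measured against the distance captured when BoostEmissive is called.
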(event Custom|BoostEmissive
  (Variables|EmissiveBoost|SetbBoostEmissive true)
  (Variables|EmissiveBoost|SetDistance (Math|Vector|VectorLength (- (Transformation|GetActorLocation) (Variables|EmissiveBoost|GetEndLocation)))))

(event EventBeginPlay
  (bind _colors (Variables|Default|GetColors))
  (bind _returnvalue (Utilities|Array|Length _colors))
  (Utilities|FlowControl|Sequence
    (:then_0
      ;[1 1 1] CALCULATE A RANDOM VELOCITY
      (Variables|Movement|SetVelocity (Math|Random|RandomFloatinRange (Variables|Movement|GetMinVelocity) (Variables|Movement|GetMaxVelocity))))
    (:then_1
      ;[1 1 1] GET A RANDOM COLOR FOR THE TEXT
      (if (> _returnvalue 0)
        (Rendering|Components|TextRender|SetTextRenderColor (Variables|Default|GetTextRender) (Math|Conversions|ToColor(LinearColor) (Utilities|Array|Get(acopy) (Variables|Default|GetColors) (Math|Random|RandomInteger _returnvalue))))))
    (:then_2
      ;[1 1 1] GET DIRECTION TO MOLE MANAGER
      (bind _outactors (Actor|GetAllActorsOfClass "/Game/Blueprints/Minigames/Mole/BP_MoleManager.BP_MoleManager_C"))
      (if (> (Utilities|Array|Length _outactors) 0)
        (Variables|EmissiveBoost|SetEndLocation (Default|GetFloatingTextTarget (Utilities|Array|Get(acopy) _outactors)))
        (Variables|Movement|SetDirection (Math|Vector|Normalize (- (Default|GetFloatingTextTarget (Utilities|Array|Get(acopy) _outactors)) (Transformation|GetActorLocation))))))))

(event EventTick
  (params (DeltaSeconds :type Float%20%28single-precision%29))
  (Utilities|FlowControl|Sequence
    (:then_0
      ;[1 1 1] MOVE THE TEXT
      (Transformation|SetActorLocation (+ (Transformation|GetActorLocation) (* (* (Variables|Movement|GetDirection) (Variables|Movement|GetVelocity)) (Utilities|Time|GetWorldDeltaSeconds))) false true))
    (:then_1
      (Rendering|Material|SetScalarParameterValue (Variables|Default|GetTextMaterial) "EmissiveIntensity" (Math|Float|Lerp (Variables|EmissiveBoost|GetMinEmissiveIntensity) (Variables|EmissiveBoost|GetMaxEmissiveIntensity) (/ (Math|Float|Absolute(Float) (- (Utilities|CurDistance) (Variables|EmissiveBoost|GetDistance))) (Variables|EmissiveBoost|GetDistance))) :!class /Script/Engine.MaterialInstanceDynamic))))

(fn ConstructionScript
  (bind _textrender (Variables|Default|GetTextRender))
  (bind _returnvalue (Rendering|Material|CreateDynamicMaterialInstance _textrender 0 (Rendering|Material|GetMaterial _textrender 0) "None" :!class /Script/Engine.PrimitiveComponent))
  (Variables|Default|SetTextMaterial _returnvalue))