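; Trigger volume actor that streams in a named level once a BP_BasePawn is inside its box.
; Each Tick runs a BoxOverlapActors query for pawns at the actor's location, sized from the Box component's scaled extent, rather than using overlap events.
; The first hit passes a DoOnce into Load Stream Level for LevelToStream, which blocks on load and shows the level afterwards.
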(event EventBeginPlay)

(event Collision|EventActorBeginOverlap
  (params (OtherActor :type Actor%20Object%20Reference)))

(event EventTick
  (params (DeltaSeconds :type Float%20%28single-precision%29))
  (bind _returnvalue (Collision|BoxOverlapActors (Transformation|GetActorLocation) (* (Variables|/Script/Engine.BoxComponent|GetBoxExtent (Variables|Default|GetBox)) (Transformation|GetWorldScale (Variables|Default|GetBox))) (Utilities|Array|MakeArray "ObjectTypeQuery3") "/Game/Blueprints/Gameplay/BP_BasePawn.BP_BasePawn_C" :!class /Script/Engine.KismetSystemLibrary))
  (if _returnvalue
    (Utilities|FlowControl|DoOnce false
      (:Completed
        (Game|LoadStreamLevel(byName) (Variables|Default|GetLevelToStream) true true)))))

(fn ConstructionScript)