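; Teleportation trace actor that sends a spinning skeletal mesh from its root to an EndPoint component, then removes itself.
; The construction script aims the mesh at EndPoint and adds a fixed local rotation offset.
; On BeginPlay, the LerpTime timeline interpolates the mesh's world location toward EndPoint while adding local yaw each update.
; When the timeline finishes, the actor waits briefly and destroys itself.
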(event EventBeginPlay
  (bind _lerp (Timeline|LerpTime Play)
    (:Update
      (Transformation|SetWorldLocation (Variables|Default|GetSkeletalMesh) (Math|Vector|Lerp(Vector) (Transformation|GetWorldLocation (Variables|Default|GetDefaultSceneRoot)) (Transformation|GetWorldLocation (Variables|Default|GetEndPoint)) _lerp) false false)
      (Transformation|AddLocalRotation (Variables|Default|GetSkeletalMesh) (Math|Rotator|MakeRotator 0.0 0.0 2.0) false false))
    (:Finished
      (Utilities|FlowControl|Delay 3.0)
      (Actor|DestroyActor))))

(event EventTick
  (params (DeltaSeconds :type Float%20%28single-precision%29)))

(fn ConstructionScript
  (bind _skeletalmesh (Variables|Default|GetSkeletalMesh))
  (bind _endpoint (Variables|Default|GetEndPoint))
  (bind _returnvalue (Transformation|GetWorldLocation _skeletalmesh))
  (bind _returnvalue_2 (Transformation|GetWorldLocation _endpoint))
  (bind _returnvalue_3 (Math|Rotator|FindLookatRotation _returnvalue _returnvalue_2))
  (Transformation|SetWorldRotation (Variables|Default|GetSkeletalMesh) (Math|Rotator|MakeRotator (.roll _returnvalue_3) (.pitch _returnvalue_3) (.yaw _returnvalue_3)) false false)
  (Transformation|AddLocalRotation (Variables|Default|GetSkeletalMesh) "0.000000,-90.000000,90.000000" false false))