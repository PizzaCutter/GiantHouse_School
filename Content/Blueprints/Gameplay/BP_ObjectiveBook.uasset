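; Objective book that the player flips by swiping the right hand sphere fast through trigger boxes, with haptic feedback.
; ABP_Book animates a skeletal page, shown only mid-flip over static pages, and flags page index changes that Tick applies.
; Four dynamic materials draw background and text from a texture array, where objectives saved in the GameInstance swap in unlocked versions.
; Tick also switches English, Dutch or French material parameters on culture changes.
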(event OnComponentBeginOverlap(BC_TurnPrev)
  (params (OverlappedComponent :type Primitive%20Component%20Object%20Reference) (OtherActor :type Actor%20Object%20Reference) (OtherComp :type Primitive%20Component%20Object%20Reference) (OtherBodyIndex :type Integer) (bFromSweep :type Boolean) (SweepResult :type Hit%20Result%20Structure%20%28by%20ref%29))
  (bind _asbp_base_pawn (Utilities|Casting|CastToBP_BasePawn OtherActor))
  (Utilities|IsValid (Variables|/Script/GiantHouseDEV.BasePawn|GetpHandSphereR _asbp_base_pawn)
    (:Is%20Valid
      (if (== OtherComp (Variables|/Script/GiantHouseDEV.BasePawn|GetpHandSphereR _asbp_base_pawn))
        (bind _output_get (Variables|Default|SetTurnPrevOverlappedComp OtherComp))
        (Variables|Default|SetTurnPrevStartLocation (Transformation|GetWorldLocation _output_get))
        (Variables|Default|SetTurnPrevTimer 0.0)
        (else
          (Variables|Default|SetTurnPrevOverlappedComp 0))))))

(event OnComponentBeginOverlap(BC_TurnNext)
  (params (OverlappedComponent :type Primitive%20Component%20Object%20Reference) (OtherActor :type Actor%20Object%20Reference) (OtherComp :type Primitive%20Component%20Object%20Reference) (OtherBodyIndex :type Integer) (bFromSweep :type Boolean) (SweepResult :type Hit%20Result%20Structure%20%28by%20ref%29))
  (bind _asbp_base_pawn (Utilities|Casting|CastToBP_BasePawn OtherActor))
  (Utilities|IsValid (Variables|/Script/GiantHouseDEV.BasePawn|GetpHandSphereR _asbp_base_pawn)
    (:Is%20Valid
      (if (== OtherComp (Variables|/Script/GiantHouseDEV.BasePawn|GetpHandSphereR _asbp_base_pawn))
        (bind _output_get (Variables|Default|SetTurnNextOverlappedComp OtherComp))
        (Variables|Default|SetTurnNextStartLocation (Transformation|GetWorldLocation _output_get))
        (Variables|Default|SetTurnNextTimer 0.0)
        (else
          (Variables|Default|SetTurnNextOverlappedComp 0))))))

(event OnComponentEndOverlap(BC_TurnPrev)
  (params (OverlappedComponent :type Primitive%20Component%20Object%20Reference) (OtherActor :type Actor%20Object%20Reference) (OtherComp :type Primitive%20Component%20Object%20Reference) (OtherBodyIndex :type Integer))
  (if (== OtherComp (Variables|Default|GetTurnPrevOverlappedComp))
    (if (>= (Math|Vector|VectorLength (/ (- (Transformation|GetWorldLocation OtherComp) (Variables|Default|GetTurnPrevStartLocation)) (Variables|Default|GetTurnPrevTimer))) (Variables|Default|GetRequiredVelocityToTurnPage))
      (CallFunction|TurnPrevPage))))

(event OnComponentEndOverlap(BC_TurnNext)
  (params (OverlappedComponent :type Primitive%20Component%20Object%20Reference) (OtherActor :type Actor%20Object%20Reference) (OtherComp :type Primitive%20Component%20Object%20Reference) (OtherBodyIndex :type Integer))
  (if (== OtherComp (Variables|Default|GetTurnNextOverlappedComp))
    (if (>= (Math|Vector|VectorLength (/ (- (Transformation|GetWorldLocation OtherComp) (Variables|Default|GetTurnNextStartLocation)) (Variables|Default|GetTurnNextTimer))) (Variables|Default|GetRequiredVelocityToTurnPage))
      (CallFunction|TurnNextPage))))

(event Custom|TurnNextPage
  (bind _animationblueprint (Variables|Default|GetAnimationBlueprint))
  (if (>= (Variables|Default|GetPageFlipDelayTimer) (Variables|Default|GetPageFlipDelay))
    (Class|MagicLeapControllerFunctionLibrary|PlayControllerHapticFeedback "Right" "Buzz" "Low")
    (bind _canturn (CallFunction|CanTurnNext))
    (if _canturn
      (if (not (and (Variables|/Game/Animations/Book/ABP_Book.ABP_Book_C|GetbTurnNext _animationblueprint) (Variables|/Game/Animations/Book/ABP_Book.ABP_Book_C|GetbTurnPrev _animationblueprint)))
        (Variables|/Game/Animations/Book/ABP_Book.ABP_Book_C|SetbTurnNext (Variables|Default|GetAnimationBlueprint) true)
        (Variables|Default|SetPageFlipDelayTimer 0.0)
        (if (and (Utilities|Array|IsValidIndex (Variables|Default|GetObjectiveBookTextures) (+ (Variables|Default|GetCurrentPage) 5)) (Utilities|Array|IsValidIndex (Variables|Default|GetObjectiveBookTextures) (+ (Variables|Default|GetCurrentPage) 7)))
          (Rendering|Material|SetTextureParameterValue (Variables|Default|GetRightPage) "Background" (Utilities|Array|Get(acopy) (Variables|Default|GetObjectiveBookTextures) (+ (Variables|Default|GetCurrentPage) 2)))
          (Rendering|Material|SetTextureParameterValue (Variables|Default|GetRightPage) "Text" (Utilities|Array|Get(acopy) (Variables|Default|GetObjectiveBookTextures) (+ (Variables|Default|GetCurrentPage) 3)))
          (Rendering|Material|SetTextureParameterValue (Variables|Default|GetLeftPage) "Background" (Utilities|Array|Get(acopy) (Variables|Default|GetObjectiveBookTextures) (+ (Variables|Default|GetCurrentPage) 4)))
          (Rendering|Material|SetTextureParameterValue (Variables|Default|GetLeftPage) "Text" (Utilities|Array|Get(acopy) (Variables|Default|GetObjectiveBookTextures) (+ (Variables|Default|GetCurrentPage) 5)))
          (Utilities|FlowControl|Delay 0.0)
          (Rendering|Material|SetTextureParameterValue (Variables|Default|GetStaticRightPage) "Background" (Utilities|Array|Get(acopy) (Variables|Default|GetObjectiveBookTextures) (+ (Variables|Default|GetCurrentPage) 6)))
          (Rendering|Material|SetTextureParameterValue (Variables|Default|GetStaticRightPage) "Text" (Utilities|Array|Get(acopy) (Variables|Default|GetObjectiveBookTextures) (+ (Variables|Default|GetCurrentPage) 7))))))))

(event Custom|TurnPrevPage
  (bind _animationblueprint (Variables|Default|GetAnimationBlueprint))
  (if (>= (Variables|Default|GetPageFlipDelayTimer) (Variables|Default|GetPageFlipDelay))
    (Class|MagicLeapControllerFunctionLibrary|PlayControllerHapticFeedback "Right" "Buzz" "Low")
    (bind _canturn (CallFunction|CanTurnPrev))
    (if _canturn
      (if (not (and (Variables|/Game/Animations/Book/ABP_Book.ABP_Book_C|GetbTurnNext _animationblueprint) (Variables|/Game/Animations/Book/ABP_Book.ABP_Book_C|GetbTurnPrev _animationblueprint)))
        (Variables|/Game/Animations/Book/ABP_Book.ABP_Book_C|SetbTurnPrev (Variables|Default|GetAnimationBlueprint) true)
        (Variables|Default|SetPageFlipDelayTimer 0.0)
        (if (and (Utilities|Array|IsValidIndex (Variables|Default|GetObjectiveBookTextures) (+ (Variables|Default|GetCurrentPage) -4)) (Utilities|Array|IsValidIndex (Variables|Default|GetObjectiveBookTextures) (+ (Variables|Default|GetCurrentPage) -3)))
          (Rendering|Material|SetTextureParameterValue (Variables|Default|GetLeftPage) "Background" (Utilities|Array|Get(acopy) (Variables|Default|GetObjectiveBookTextures) (+ (Variables|Default|GetCurrentPage) 0)))
          (Rendering|Material|SetTextureParameterValue (Variables|Default|GetLeftPage) "Text" (Utilities|Array|Get(acopy) (Variables|Default|GetObjectiveBookTextures) (+ (Variables|Default|GetCurrentPage) 1)))
          (Rendering|Material|SetTextureParameterValue (Variables|Default|GetRightPage) "Background" (Utilities|Array|Get(acopy) (Variables|Default|GetObjectiveBookTextures) (+ (Variables|Default|GetCurrentPage) -2)))
          (Rendering|Material|SetTextureParameterValue (Variables|Default|GetRightPage) "Text" (Utilities|Array|Get(acopy) (Variables|Default|GetObjectiveBookTextures) (+ (Variables|Default|GetCurrentPage) -1)))
          (Utilities|FlowControl|Delay 0.0)
          (Rendering|Material|SetTextureParameterValue (Variables|Default|GetStaticLeftPage) "Background" (Utilities|Array|Get(acopy) (Variables|Default|GetObjectiveBookTextures) (+ (Variables|Default|GetCurrentPage) -4)))
          (Rendering|Material|SetTextureParameterValue (Variables|Default|GetStaticLeftPage) "Text" (Utilities|Array|Get(acopy) (Variables|Default|GetObjectiveBookTextures) (+ (Variables|Default|GetCurrentPage) -3))))))))

(event Custom|SkeletalMeshVisibilityCheck
  (bind _animationblueprint (Variables|Default|GetAnimationBlueprint))
  (if (or (Variables|/Game/Animations/Book/ABP_Book.ABP_Book_C|GetbTurnNext _animationblueprint) (Variables|/Game/Animations/Book/ABP_Book.ABP_Book_C|GetbTurnPrev _animationblueprint))
    (Rendering|SetVisibility (Variables|Default|GetSKM_BookPage) true false)
    (else
      (Rendering|SetVisibility (Variables|Default|GetSKM_BookPage) false false))))

(event EventBeginPlay
  ;[1 1 1] CACHE THE ANIMATION BLUEPRINT
  (Utilities|FlowControl|Sequence
    (:then_0
      (bind _asabp_book (Utilities|Casting|CastToABP_Book (Components|SkeletalMesh|GetAnimInstance (Variables|Default|GetSKM_BookPage))))
      (Variables|Default|SetAnimationBlueprint _asabp_book))
    (:then_1
      (CallFunction|LoadInfo))))

(event EventTick
  (params (DeltaSeconds :type Float%20%28single-precision%29))
  (bind _returnvalue (Utilities|Internationalization|GetCurrentCulture))
  (Utilities|FlowControl|Sequence
    (:then_0
      (if (Variables|/Game/Animations/Book/ABP_Book.ABP_Book_C|GetbIncreasePageIndex (Variables|Default|GetAnimationBlueprint))
        (Variables|/Game/Animations/Book/ABP_Book.ABP_Book_C|SetbIncreasePageIndex (Variables|Default|GetAnimationBlueprint) false)
        (Variables|Default|SetCurrentPage (+ (Variables|Default|GetCurrentPage) 4))
        (CallFunction|UpdatePages)))
    (:then_1
      (if (Variables|/Game/Animations/Book/ABP_Book.ABP_Book_C|GetbDecreasePageIndex (Variables|Default|GetAnimationBlueprint))
        (Variables|/Game/Animations/Book/ABP_Book.ABP_Book_C|SetbDecreasePageIndex (Variables|Default|GetAnimationBlueprint) false)
        (Variables|Default|SetCurrentPage (+ (Variables|Default|GetCurrentPage) -4))
        (CallFunction|UpdatePages)))
    (:then_2
      (CallFunction|SkeletalMeshVisibilityCheck))
    (:then_3
      (Variables|Default|SetTurnPrevTimer (+ (Variables|Default|GetTurnPrevTimer) (Utilities|Time|GetWorldDeltaSeconds)))
      (Variables|Default|SetTurnNextTimer (+ (Variables|Default|GetTurnNextTimer) (Utilities|Time|GetWorldDeltaSeconds)))
      (Variables|Default|SetPageFlipDelayTimer (+ (Variables|Default|GetPageFlipDelayTimer) (Utilities|Time|GetWorldDeltaSeconds))))
    (:then_4
      (if (Utilities|Enum|NotEqual(Enum) (Variables|Default|GetPrevLanguage) _returnvalue)
        (Variables|Default|SetPrevLanguage _returnvalue)
        (CallFunction|ChangeLanguage)))
    (:then_5
      (Development|PrintString (Utilities|String|ToString(Integer) (Variables|Default|GetCurrentPage)) true true "(R=0.000000,G=0.660000,B=1.000000,A=1.000000)" 0.0))))

(fn ConstructionScript
  (Utilities|FlowControl|Sequence
    (:then_0
      (bind _returnvalue (Rendering|Material|CreateDynamicMaterialInstance "/Game/Materials/ObjectiveBook/MAT_Book_Inst.MAT_Book_Inst" "None" :!class /Script/Engine.KismetMaterialLibrary))
      (Variables|Default|SetStaticLeftPage _returnvalue)
      (bind _returnvalue_2 (Rendering|Material|CreateDynamicMaterialInstance "/Game/Materials/ObjectiveBook/MAT_Book_Inst.MAT_Book_Inst" "None" :!class /Script/Engine.KismetMaterialLibrary))
      (Variables|Default|SetStaticRightPage _returnvalue_2)
      (bind _returnvalue_3 (Rendering|Material|CreateDynamicMaterialInstance "/Game/Materials/ObjectiveBook/MAT_Book_Inst.MAT_Book_Inst" "None" :!class /Script/Engine.KismetMaterialLibrary))
      (Variables|Default|SetLeftPage _returnvalue_3)
      (bind _returnvalue_4 (Rendering|Material|CreateDynamicMaterialInstance "/Game/Materials/ObjectiveBook/MAT_Book_Inst.MAT_Book_Inst" "None" :!class /Script/Engine.KismetMaterialLibrary))
      (Variables|Default|SetRightPage _returnvalue_4))
    (:then_1
      (Rendering|Material|SetMaterial (Variables|Default|GetSM_BookStaticPages) 0 (Variables|Default|GetStaticLeftPage))
      (Rendering|Material|SetMaterial (Variables|Default|GetSM_BookStaticPages) 1 (Variables|Default|GetStaticRightPage)))
    (:then_2
      (Rendering|Material|SetMaterial (Variables|Default|GetSKM_BookPage) 0 (Variables|Default|GetLeftPage))
      (Rendering|Material|SetMaterial (Variables|Default|GetSKM_BookPage) 1 (Variables|Default|GetRightPage)))
    (:then_3
      (CallFunction|UpdatePages)
      (CallFunction|ChangeLanguage))))

(fn CanTurnNext
  (return (and (Utilities|Array|IsValidIndex (Variables|Default|GetObjectiveBookTextures) (+ (Variables|Default|GetCurrentPage) 4)) (Rendering|IsVisible (Variables|Default|GetDefaultSceneRoot)))))

(fn UpdatePages
  (if (Utilities|Array|IsValidIndex (Variables|Default|GetObjectiveBookTextures) (+ (Variables|Default|GetCurrentPage) 5))
    (Utilities|FlowControl|Sequence
      (:then_0
        ;[1 1 1] STATIC PAGES
        (Rendering|Material|SetTextureParameterValue (Variables|Default|GetStaticLeftPage) "Background" (Utilities|Array|Get(acopy) (Variables|Default|GetObjectiveBookTextures) (Variables|Default|GetCurrentPage)))
        (Rendering|Material|SetTextureParameterValue (Variables|Default|GetStaticLeftPage) "Text" (Utilities|Array|Get(acopy) (Variables|Default|GetObjectiveBookTextures) (+ (Variables|Default|GetCurrentPage) 1)))
        (Rendering|Material|SetTextureParameterValue (Variables|Default|GetStaticRightPage) "Background" (Utilities|Array|Get(acopy) (Variables|Default|GetObjectiveBookTextures) (+ (Variables|Default|GetCurrentPage) 2)))
        (Rendering|Material|SetTextureParameterValue (Variables|Default|GetStaticRightPage) "Text" (Utilities|Array|Get(acopy) (Variables|Default|GetObjectiveBookTextures) (+ (Variables|Default|GetCurrentPage) 3))))
      (:then_1
        (Rendering|Material|SetTextureParameterValue (Variables|Default|GetRightPage) "Background" (Utilities|Array|Get(acopy) (Variables|Default|GetObjectiveBookTextures) (+ (Variables|Default|GetCurrentPage) 2)))
        (Rendering|Material|SetTextureParameterValue (Variables|Default|GetRightPage) "Text" (Utilities|Array|Get(acopy) (Variables|Default|GetObjectiveBookTextures) (+ (Variables|Default|GetCurrentPage) 3))))
      (:then_2
        (Rendering|Material|SetTextureParameterValue (Variables|Default|GetLeftPage) "Background" (Utilities|Array|Get(acopy) (Variables|Default|GetObjectiveBookTextures) (+ (Variables|Default|GetCurrentPage) 4)))
        (Rendering|Material|SetTextureParameterValue (Variables|Default|GetLeftPage) "Text" (Utilities|Array|Get(acopy) (Variables|Default|GetObjectiveBookTextures) (+ (Variables|Default|GetCurrentPage) 5)))))))

(fn CanTurnPrev
  (return (and (Utilities|Array|IsValidIndex (Variables|Default|GetObjectiveBookTextures) (+ (Variables|Default|GetCurrentPage) -4)) (Rendering|IsVisible (Variables|Default|GetDefaultSceneRoot)))))

(fn UnlockInfo
  (params (ObjectiveInfoToUnlock :type eOBJECTIVEBOOKINFO%20Enum :default "NewEnumerator0"))
  (bind _returnvalue (Math|Conversions|ToInteger(Byte) ObjectiveInfoToUnlock))
  (bind _returnvalue_2 (* _returnvalue 4))
  (bind _returnvalue_3 (+ _returnvalue_2 4))
  (bind _returnvalue_4 (+ _returnvalue_3 3))
  (bind _returnvalue_5 (+ _returnvalue_3 1))
  (Utilities|Array|SetArrayElem (Variables|Default|GetObjectiveBookTextures) _returnvalue_5 (Utilities|Array|Get(acopy) (Variables|Default|GetObjectiveBookTexturesUnlocked) _returnvalue_5))
  (Utilities|Array|SetArrayElem (Variables|Default|GetObjectiveBookTextures) _returnvalue_4 (Utilities|Array|Get(acopy) (Variables|Default|GetObjectiveBookTexturesUnlocked) _returnvalue_4))
  (CallFunction|UpdatePages))

(fn LoadInfo
  (bind _asbp_game_instance (Utilities|Casting|CastToBP_GameInstance (Game|GetGameInstance)))
  (for _array_element (Variables|/Game/Blueprints/BP_GameInstance.BP_GameInstance_C|GetUnlockedInfo _asbp_game_instance)
    (CallFunction|UnlockInfo _array_element)))

(fn ChangeLanguage
  (Utilities|FlowControl|Sequence
    (:then_0
      (Rendering|Material|SetScalarParameterValue (Variables|Default|GetStaticLeftPage) "Dutch" 0.0 :!class /Script/Engine.MaterialInstanceDynamic)
      (Rendering|Material|SetScalarParameterValue (Variables|Default|GetStaticLeftPage) "English" 0.0 :!class /Script/Engine.MaterialInstanceDynamic)
      (Rendering|Material|SetScalarParameterValue (Variables|Default|GetStaticLeftPage) "French" 0.0 :!class /Script/Engine.MaterialInstanceDynamic)
      (switch string (Variables|Default|GetPrevLanguage)
        (:Default
          (Rendering|Material|SetScalarParameterValue (Variables|Default|GetStaticLeftPage) "English" 1.0 :!class /Script/Engine.MaterialInstanceDynamic :!label _label))
        (:en
          (goto _label))
        (:nl-BE
          (Rendering|Material|SetScalarParameterValue (Variables|Default|GetStaticLeftPage) "Dutch" 1.0 :!class /Script/Engine.MaterialInstanceDynamic))
        (:fr
          (Rendering|Material|SetScalarParameterValue (Variables|Default|GetStaticLeftPage) "French" 1.0 :!class /Script/Engine.MaterialInstanceDynamic))))
    (:then_1
      (Rendering|Material|SetScalarParameterValue (Variables|Default|GetStaticRightPage) "Dutch" 0.0 :!class /Script/Engine.MaterialInstanceDynamic)
      (Rendering|Material|SetScalarParameterValue (Variables|Default|GetStaticRightPage) "English" 0.0 :!class /Script/Engine.MaterialInstanceDynamic)
      (Rendering|Material|SetScalarParameterValue (Variables|Default|GetStaticRightPage) "French" 0.0 :!class /Script/Engine.MaterialInstanceDynamic)
      (switch string (Variables|Default|GetPrevLanguage)
        (:Default
          (Rendering|Material|SetScalarParameterValue (Variables|Default|GetStaticRightPage) "English" 1.0 :!class /Script/Engine.MaterialInstanceDynamic :!label _label_2))
        (:en
          (goto _label_2))
        (:nl-BE
          (Rendering|Material|SetScalarParameterValue (Variables|Default|GetStaticRightPage) "Dutch" 1.0 :!class /Script/Engine.MaterialInstanceDynamic))
        (:fr
          (Rendering|Material|SetScalarParameterValue (Variables|Default|GetStaticRightPage) "French" 1.0 :!class /Script/Engine.MaterialInstanceDynamic))))
    (:then_2
      (Rendering|Material|SetScalarParameterValue (Variables|Default|GetLeftPage) "Dutch" 0.0 :!class /Script/Engine.MaterialInstanceDynamic)
      (Rendering|Material|SetScalarParameterValue (Variables|Default|GetLeftPage) "English" 0.0 :!class /Script/Engine.MaterialInstanceDynamic)
      (Rendering|Material|SetScalarParameterValue (Variables|Default|GetLeftPage) "French" 0.0 :!class /Script/Engine.MaterialInstanceDynamic)
      (switch string (Variables|Default|GetPrevLanguage)
        (:Default
          (Rendering|Material|SetScalarParameterValue (Variables|Default|GetLeftPage) "English" 1.0 :!class /Script/Engine.MaterialInstanceDynamic :!label _label_3))
        (:en
          (goto _label_3))
        (:nl-BE
          (Rendering|Material|SetScalarParameterValue (Variables|Default|GetLeftPage) "Dutch" 1.0 :!class /Script/Engine.MaterialInstanceDynamic))
        (:fr
          (Rendering|Material|SetScalarParameterValue (Variables|Default|GetLeftPage) "French" 1.0 :!class /Script/Engine.MaterialInstanceDynamic))))
    (:then_3
      (Rendering|Material|SetScalarParameterValue (Variables|Default|GetRightPage) "Dutch" 0.0 :!class /Script/Engine.MaterialInstanceDynamic)
      (Rendering|Material|SetScalarParameterValue (Variables|Default|GetRightPage) "English" 0.0 :!class /Script/Engine.MaterialInstanceDynamic)
      (Rendering|Material|SetScalarParameterValue (Variables|Default|GetRightPage) "French" 0.0 :!class /Script/Engine.MaterialInstanceDynamic)
      (switch string (Variables|Default|GetPrevLanguage)
        (:Default
          (Rendering|Material|SetScalarParameterValue (Variables|Default|GetRightPage) "English" 1.0 :!class /Script/Engine.MaterialInstanceDynamic :!label _label_4))
        (:en
          (goto _label_4))
        (:nl-BE
          (Rendering|Material|SetScalarParameterValue (Variables|Default|GetRightPage) "Dutch" 1.0 :!class /Script/Engine.MaterialInstanceDynamic))
        (:fr
          (Rendering|Material|SetScalarParameterValue (Variables|Default|GetRightPage) "French" 1.0 :!class /Script/Engine.MaterialInstanceDynamic))))))