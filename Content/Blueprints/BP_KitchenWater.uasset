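; BP_KitchenWater is a kitchen water hazard that stays hidden until Start triggers a filling sequence, then reacts to the radio.
; Timelines scale the stream, raise the surface and splash, then lower and remove the stream, setting Filled, while a dynamic material swaps the displacement texture.
; Once filled, radio contact swaps its audio.
; If the radio is held on first contact, the player is electrified, the screen fades and the death level loads.
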(event OnComponentBeginOverlap(Radio)
  (params (OverlappedComponent :type Primitive%20Component%20Object%20Reference) (OtherActor :type Actor%20Object%20Reference) (OtherComp :type Primitive%20Component%20Object%20Reference) (OtherBodyIndex :type Integer) (bFromSweep :type Boolean) (SweepResult :type Hit%20Result%20Structure%20%28by%20ref%29))
  (if (Variables|Default|GetbFilled)
    (bind _asbp_radio (Utilities|Casting|CastToBP_Radio OtherActor))
    (bind _asaudio_component (Utilities|Casting|CastToAudioComponent (Components|GetChildComponent (Variables|/Script/Engine.StaticMeshActor|GetStaticMeshComponent _asbp_radio) 1)))
    (Audio|Components|Audio|Stop _asaudio_component)
    (if (not (Variables|Default|GetbPlayedAudio))
      (Audio|SpawnSoundAttached "/Game/Audio/AMB/AMB_RobbeMusic.AMB_RobbeMusic" (Variables|/Script/Engine.StaticMeshActor|GetStaticMeshComponent _asbp_radio) "None" "0, 0, 0" "0, 0, 0" "KeepRelativeOffset" false 0.05 1.0 0.0 "/Game/Audio/SA_DefautlFallOff.SA_DefautlFallOff" 0)
      (Variables|Default|SetbPlayedAudio true)
      (if (Variables|/Game/Blueprints/InteractiveElements/BP_Radio.BP_Radio_C|GetbIsPickedUp _asbp_radio)
        (bind _asbp_game_instance (Utilities|Casting|CastToBP_GameInstance (Game|GetGameInstance)))
        (Default|StartElectrification (Variables|/Game/Blueprints/BP_GameInstance.BP_GameInstance_C|GetBasePawn _asbp_game_instance) "NewEnumerator0")
        (Default|SavePawnLocation _asbp_game_instance)
        (Utilities|FlowControl|Delay (Variables|/Game/Blueprints/BP_GameInstance.BP_GameInstance_C|GetHazardKillTime _asbp_game_instance))
        (CameraFades|StartCameraFade (Game|GetPlayerCameraManager 0) 0.0 1.0 (Variables|/Game/Blueprints/BP_GameInstance.BP_GameInstance_C|GetFadeTime _asbp_game_instance) "(R=1.000000,G=1.000000,B=1.000000,A=1.000000)" false true)
        (Utilities|FlowControl|Delay (Variables|/Game/Blueprints/BP_GameInstance.BP_GameInstance_C|GetFadeTime _asbp_game_instance))
        (Variables|/Game/Blueprints/BP_GameInstance.BP_GameInstance_C|SetLevelLoadOptions _asbp_game_instance "Radio")
        (Game|OpenLevel(byName) "MAP_PlayerDeadScene")))))

(event Custom|Start
  (bind _plane (Variables|Default|GetPlane))
  (bind _stream (Variables|Default|GetStream))
  (bind _splash (Variables|Default|GetSplash))
  (bind _returnvalue (Audio|SpawnSoundatLocation "/Game/Audio/SFX/SFX_WaterRunning.SFX_WaterRunning" (Transformation|GetActorLocation) "0, 0, 0" 0.5 1.0 0.0 "/Game/Audio/SA_DefautlFallOff.SA_DefautlFallOff" 0))
  (Variables|Default|SetWaterRunning _returnvalue)
  (Rendering|SetVisibility (Variables|Default|GetDefaultSceneRoot) true true)
  (Utilities|FlowControl|Sequence
    (:then_0
      (Rendering|SetVisibility (Variables|Default|GetSplash) false false)
      ;[1 1 1] Stream Down
      (bind _scale (Timeline|Scale Play)
        (:Update
          (Transformation|SetRelativeScale3D (Variables|Default|GetStream) _scale))))
    (:then_1
      (Utilities|FlowControl|Delay 0.1)
      ;[1 1 1] Raise Water
      (Rendering|SetVisibility _splash true false)
      (bind _move_up (Timeline|Raise%20Water Play)
        (:Update
          (Transformation|SetRelativeLocation (Variables|Default|GetPlane) _move_up false false)
          (Transformation|SetRelativeLocation _splash _move_up false false))))
    (:then_2
      (Utilities|FlowControl|Delay 9.5)
      ;[1 1 1] Stream Delete
      (Utilities|FlowControl|Sequence
        (:then_0
          (bind _move_down (Timeline|lower%20stream Play)
            (:Update
              (Transformation|SetRelativeLocation _stream _move_down false false))
            (:Finished
              (Components|DestroyComponent _stream)
              (Rendering|SetVisibility (Variables|Default|GetSplash) false false)
              (Audio|Components|Audio|Stop (Variables|Default|GetWaterRunning))
              (Variables|Default|SetbFilled true))))
        (:then_1
          ;[1 1 1] Change Material
          (bind _returnvalue_2 (Rendering|Material|CreateDynamicMaterialInstance (Rendering|Material|GetMaterial _plane 0) "None" :!class /Script/Engine.KismetMaterialLibrary))
          (Rendering|Material|SetMaterial _plane 0 _returnvalue_2)
          (Rendering|Material|SetTextureParameterValue _returnvalue_2 "Displacement Texture" "/Engine/Functions/Engine_MaterialFunctions02/ExampleContent/Textures/LowResBlurredNoise.LowResBlurredNoise"))))))

(fn ConstructionScript
  (Rendering|SetVisibility (Variables|Default|GetDefaultSceneRoot) false true))