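; BP_Drawer is an interactive drawer; this graph handles its closing and bounce sounds on Tick.
; When JustBounced is set with enough velocity, it plays a random-pitch close sound, gated by a DoOnce that resets after a short delay.
; While dragged, a second DoOnce plays the same sound at the closed position and re-arms once pulled out a tenth of DrawerLength.
; The movement itself is not driven here.
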(event EventBeginPlay)

(event Collision|EventActorBeginOverlap
  (params (OtherActor :type Actor%20Object%20Reference)))

(event EventTick
  (params (DeltaSeconds :type Float%20%28single-precision%29))
  (Utilities|FlowControl|Sequence
    (:then_0
      (if (and (>= (Math|Float|Absolute(Float) (Variables|Default|GetInitialVelocity)) 1.0) (Variables|Default|GetbJustBounced))
        (Utilities|FlowControl|DoOnce false :!label _label
          (:Completed
            (Audio|PlaySoundatLocation "/Game/Audio/SFX/SFX_ClosetCloseSound_Cue.SFX_ClosetCloseSound_Cue" (Transformation|GetActorLocation) "0, 0, 0" 1.0 (Math|Random|RandomFloatinRange 0.8 1.2) 0.0 0 0 0)
            (Development|PrintString "BOUNCED" false false)
            (Utilities|FlowControl|Delay 0.5)
            (goto _label Reset)))))
    (:then_1
      (if (Variables|Default|GetbIsBeingDragged)
        (Utilities|FlowControl|Sequence
          (:then_0
            (if (<= (.x (Variables|/Script/Engine.SceneComponent|GetRelativeLocation (Variables|Default|GetpDrawer))) (.x (Variables|Default|GetInitialLocation)))
              (Utilities|FlowControl|DoOnce false :!label _label_2
                (:Completed
                  (Audio|PlaySoundatLocation "/Game/Audio/SFX/SFX_ClosetCloseSound_Cue.SFX_ClosetCloseSound_Cue" (Transformation|GetActorLocation) "0, 0, 0" 1.0 (Math|Random|RandomFloatinRange 0.8 1.2) 0.0 0 0 0)
                  (Development|PrintString "BOUNCED" false false)))))
          (:then_1
            (if (>= (.x (Variables|/Script/Engine.SceneComponent|GetRelativeLocation (Variables|Default|GetpDrawer))) (+ (.x (Variables|Default|GetInitialLocation)) (/ (Variables|Default|GetDrawerLength) 1e+01)))
              (goto _label_2 Reset))))))))

(fn ConstructionScript)