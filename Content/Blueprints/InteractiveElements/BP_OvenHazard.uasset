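; BP_OvenHazard is an oven hazard that burns the player's hand on contact and leads to death.
; A box overlap checks for either hand sphere of BP_BasePawn, saves the pawn location through BP_GameInstance and, unless already dying, starts that hand's burn.
; It then marks the pawn dying, waits, fades the camera out and opens MAP_PlayerDeadScene with "Oven" stored in the game instance's level load options.
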(event OnComponentBeginOverlap(Box)
  (params (OverlappedComponent :type Primitive%20Component%20Object%20Reference) (OtherActor :type Actor%20Object%20Reference) (OtherComp :type Primitive%20Component%20Object%20Reference) (OtherBodyIndex :type Integer) (bFromSweep :type Boolean) (SweepResult :type Hit%20Result%20Structure%20%28by%20ref%29))
  (bind _asbp_base_pawn (Utilities|Casting|CastToBP_BasePawn OtherActor))
  (Utilities|IsValid (Variables|/Script/GiantHouseDEV.BasePawn|GetpHandSphereL _asbp_base_pawn)
    (:Is%20Valid
      (Utilities|IsValid (Variables|/Script/GiantHouseDEV.BasePawn|GetpHandSphereR _asbp_base_pawn)
        (:Is%20Valid
          (if (or (== (Variables|/Script/GiantHouseDEV.BasePawn|GetpHandSphereL _asbp_base_pawn) OtherComp) (== (Variables|/Script/GiantHouseDEV.BasePawn|GetpHandSphereR _asbp_base_pawn) OtherComp))
            (bind _asbp_game_instance (Utilities|Casting|CastToBP_GameInstance (Game|GetGameInstance)))
            (Default|SavePawnLocation _asbp_game_instance)
            (if (not (Class|BasePawn|IsDying (Variables|/Game/Blueprints/BP_GameInstance.BP_GameInstance_C|GetBasePawn _asbp_game_instance)))
              (if (== (Variables|/Script/GiantHouseDEV.BasePawn|GetpHandSphereL _asbp_base_pawn) OtherComp)
                (Utilities|FlowControl|DoOnce false
                  (:Completed
                    (Default|StartBurn _asbp_base_pawn "NewEnumerator0")))
                (else
                  (Utilities|FlowControl|DoOnce false
                    (:Completed
                      (Default|StartBurn _asbp_base_pawn "NewEnumerator1")))))
              (bind _asbp_game_instance_2 (Utilities|Casting|CastToBP_GameInstance (Game|GetGameInstance)))
              (Class|BasePawn|SetDying (Variables|/Game/Blueprints/BP_GameInstance.BP_GameInstance_C|GetBasePawn _asbp_game_instance_2) true)
              (Utilities|FlowControl|Delay 5.0)
              (CameraFades|StartCameraFade :self (Game|GetPlayerCameraManager 0) :ToAlpha 1.0 :Duration 1.0)
              (Utilities|FlowControl|Delay 1.0)
              (Variables|/Game/Blueprints/BP_GameInstance.BP_GameInstance_C|SetLevelLoadOptions _asbp_game_instance_2 "Oven")
              (Game|OpenLevel(byName) "MAP_PlayerDeadScene"))))))))

(event EventBeginPlay)

(event Collision|EventActorBeginOverlap
  (params (OtherActor :type Actor%20Object%20Reference)))

(event EventTick
  (params (DeltaSeconds :type Float%20%28single-precision%29)))

(fn ConstructionScript)