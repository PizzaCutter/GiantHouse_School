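; Draggable door that, once swung to its open arrow, streams or opens a level, with special names for quitting or reloading after death.
; While held, its opening angle drives plane glow and a white camera fade.
; Streamed or unnamed targets reset the door, teleport the player to SpawnLocation, fade back in, unload listed levels and reset teleport areas.
; Tick also swings the door shut when nearly still, unless disabled.
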(event Custom|Reset
  (Transformation|SetRelativeRotation (Variables|Default|GetpDoorRotator) (Math|Rotator|MakeRotator 0.0 0.0 (Variables|Default|GetInitialYaw)) false false)
  (Utilities|FlowControl|DoOnce false) ; enters at Reset
)

(event EventBeginPlay
  (|CallParentFunction)
  (Variables|Default|SetInitialYaw (.yaw (.rotation (Transformation|GetRelativeTransform (Variables|Default|GetpDoorRotator))))))

(event EventTick
  (params (DeltaSeconds :type Float%20%28single-precision%29))
  (bind _pdoorrotator (Variables|Default|GetpDoorRotator))
  (bind _openarrow (Variables|Default|GetOpenArrow))
  (bind _pdoorrotator_2 (Variables|Default|GetpDoorRotator))
  (bind _initialyaw (Variables|Default|GetInitialYaw))
  (bind _relativerotation (Variables|/Script/Engine.SceneComponent|GetRelativeRotation _pdoorrotator))
  (bind _relativerotation_2 (Variables|/Script/Engine.SceneComponent|GetRelativeRotation _openarrow))
  (bind _relativerotation_3 (Variables|/Script/Engine.SceneComponent|GetRelativeRotation _pdoorrotator_2))
  (bind _returnvalue (- (.yaw _relativerotation) _initialyaw))
  (bind _returnvalue_2 (/ _returnvalue (.yaw _relativerotation_2)))
  (|CallParentFunction DeltaSeconds)
  (Utilities|FlowControl|Sequence
    (:then_0
      (if (>= (.yaw (Variables|/Script/Engine.SceneComponent|GetRelativeRotation (Variables|Default|GetpDoorRotator))) (.yaw (Variables|/Script/Engine.SceneComponent|GetRelativeRotation (Variables|Default|GetOpenArrow))))
        (Utilities|FlowControl|DoOnce false
          (:Completed
            (Variables|Default|SetbHoldingDoor false)
            (if (Utilities|Name|NotEqual(Name) (Variables|Default|GetLevelToLoad) "Dead")
              (if (Utilities|Name|NotEqual(Name) (Variables|Default|GetLevelToLoad) "Quit")
                ;[1 1 1] IF LEVEL NAME IS VALID LOAD THE LEVEL
                (if (Utilities|Name|NotEqual(Name) (Variables|Default|GetLevelToLoad) "None")
                  (if (Variables|Default|GetbToStream)
                    (Game|LoadStreamLevel(byName) (Variables|Default|GetLevelToLoad) true)
                    (CallFunction|Reset :!label _label)
                    ;[1 1 1] Teleport player to new level
                    (Transformation|SetActorLocation (Game|Player|GetPlayerPawn 0) (Transformation|GetWorldLocation (Variables|Default|GetSpawnLocation)) false false)
                    ;[1 1 1] Unfade camera
                    (bind _asbp_game_instance (Utilities|Casting|CastToBP_GameInstance (Game|GetGameInstance)))
                    (CameraFades|StartCameraFade (Game|GetPlayerCameraManager 0) 1.0 0.0 (Variables|/Game/Blueprints/BP_GameInstance.BP_GameInstance_C|GetFadeTime _asbp_game_instance) "(R=1.000000,G=1.000000,B=1.000000,A=1.000000)" false false)
                    (Utilities|FlowControl|Delay (Variables|/Game/Blueprints/BP_GameInstance.BP_GameInstance_C|GetFadeTime _asbp_game_instance))
                    (Utilities|FlowControl|Sequence
                      (:then_0
                        ;[1 1 1] UNLOAD LEVELS
                        (if (== (Utilities|Array|Length (Variables|Default|GetLevelToUnload)) 6)
                          (Game|UnloadStreamLevel(byName) (Utilities|Array|Get(acopy) (Variables|Default|GetLevelToUnload)) false)
                          (Game|UnloadStreamLevel(byName) (Utilities|Array|Get(acopy) (Variables|Default|GetLevelToUnload) 1) false)
                          (Game|UnloadStreamLevel(byName) (Utilities|Array|Get(acopy) (Variables|Default|GetLevelToUnload) 2) false)
                          (Game|UnloadStreamLevel(byName) (Utilities|Array|Get(acopy) (Variables|Default|GetLevelToUnload) 3) false)
                          (Game|UnloadStreamLevel(byName) (Utilities|Array|Get(acopy) (Variables|Default|GetLevelToUnload) 4) false)
                          (Game|UnloadStreamLevel(byName) (Utilities|Array|Get(acopy) (Variables|Default|GetLevelToUnload) 5) false)))
                      (:then_1
                        ;[1 1 1] RESET TELEPORTAREAS
                        (bind _asbase_pawn (Utilities|Casting|CastToBasePawn (Game|Player|GetPlayerPawn 0)))
                        (Class|BasePawn|ResetTeleporter _asbase_pawn)))
                    (else
                      (Game|OpenLevel(byName) (Variables|Default|GetLevelToLoad))))
                  (else
                    (goto _label)))
                (else
                  (Game|QuitGame (Game|GetPlayerController 0) "Quit" false)))
              (else
                (bind _asbp_game_instance_2 (Utilities|Casting|CastToBP_GameInstance (Game|GetGameInstance)))
                (Variables|/Game/Blueprints/BP_GameInstance.BP_GameInstance_C|SetTeleportPlayer _asbp_game_instance_2 true)
                (Game|OpenLevel(byName) (Variables|/Game/Blueprints/BP_GameInstance.BP_GameInstance_C|GetDiedLevel _asbp_game_instance_2))))))))
    (:then_1
      ;[1 1 1] SET EMISSIVE INTENSITY BASED ON OPENING OF DOOR
      (if (Variables|Default|GetbHoldingDoor)
        (if (not (Variables|Default|GetbStop))
          (Rendering|Material|SetScalarParameterValue (Variables|Default|GetEmissiveMaterial) "EmissiveIntensity" (Math|Float|Lerp (Variables|Default|GetMinEmissive) (Variables|Default|GetMaxEmissive) _returnvalue_2) :!class /Script/Engine.MaterialInstanceDynamic)
          (Class|PlayerCameraManager|SetManualCameraFade (Game|GetPlayerCameraManager 0) _returnvalue_2 "(R=1.000000,G=1.000000,B=1.000000,A=1.000000)" false))))
    (:then_2
      ;[1 1 1] ROTATE THE DOOR BACK
      (if (and (<= (Math|Float|Absolute(Float) (Variables|Default|GetInitialYawVelocity)) 1.0) (not (Variables|Default|GetbDisableAutomaticClosing)))
        (if (> (.yaw (Variables|/Script/Engine.SceneComponent|GetRelativeRotation (Variables|Default|GetpDoorRotator))) (Variables|Default|GetInitialYaw))
          (Transformation|AddRelativeRotation (Variables|Default|GetpDoorRotator) (Math|Rotator|MakeRotator 0.0 0.0 -1.0) false false)
          (else
            (Transformation|SetRelativeRotation (Variables|Default|GetpDoorRotator) (Math|Rotator|MakeRotator (.roll _relativerotation_3) (.pitch _relativerotation_3) (Variables|Default|GetInitialYaw)) false false)))))))

(fn ConstructionScript
  (bind _plane (Variables|Default|GetPlane))
  (|CallParentFunction)
  (bind _returnvalue (Rendering|Material|CreateDynamicMaterialInstance _plane 0 (Rendering|Material|GetMaterial _plane 0) "None" :!class /Script/Engine.PrimitiveComponent))
  (Variables|Default|SetEmissiveMaterial _returnvalue))

(fn OnDragStart
  (params (interactor :type World%20Interactor%20Object%20Reference))
  (bind _returnvalue (|CallParentFunction interactor))
  (bind _output_get (Variables|Default|SetbStop _returnvalue))
  (Variables|Default|SetbHoldingDoor true)
  (return _output_get))

(fn OnDragStop
  (params (interactor :type World%20Interactor%20Object%20Reference))
  (bind _returnvalue (|CallParentFunction interactor))
  (bind _output_get (Variables|Default|SetbStop _returnvalue))
  (Variables|Default|SetbHoldingDoor false)
  (return _output_get))