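; BP_Slider is a 3D UI slider that turns the X position of its PDrawer component into a displayed number.
; BeginPlay records the drawer's start and derives the end from DrawerLength.
; GetValue divides relative X by that travel, without subtracting the start, and inverts it to lerp between MinValue and MaxValue.
; Tick writes the value to TextRender as a signed, one-decimal number.
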(event EventBeginPlay
  (Variables|Default|SetStartPosition (.x (Variables|/Script/Engine.SceneComponent|GetRelativeLocation (Variables|Default|GetpDrawer))))
  (Variables|Default|SetEndPosition (+ (Variables|Default|GetStartPosition) (Variables|Default|GetDrawerLength))))

(event EventTick
  (params (DeltaSeconds :type Float%20%28single-precision%29))
  (Rendering|Components|TextRender|SetText (Variables|Default|GetTextRender) (Utilities|Text|ToText(Float) (CallFunction|GetValue) "HalfToEven" true true 1 324 1 1)))

(fn ConstructionScript)

(fn GetValue
  (return (Math|Float|Lerp (Variables|Default|GetMinValue) (Variables|Default|GetMaxValue) (- 1.0 (/ (.x (Variables|/Script/Engine.SceneComponent|GetRelativeLocation (Variables|Default|GetpDrawer))) (- (Variables|Default|GetEndPosition) (Variables|Default|GetStartPosition)))))))