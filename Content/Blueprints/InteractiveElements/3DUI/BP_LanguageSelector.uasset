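; BP_LanguageSelector is a 3D UI actor that makes English, Dutch and French toggle boxes act as a single-choice selector.
; BeginPlay gathers the BP_ToggleBox child actors into an array and enlarges any active one.
; Tick polls their HasChanged flags, then enables and enlarges the changed box while disabling and resetting the scale of the others.
; It contains no language-switching logic itself.
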(event EventBeginPlay
  (bind _asbp_toggle_box (Utilities|Casting|CastToBP_ToggleBox (Variables|/Script/Engine.ChildActorComponent|GetChildActor (Variables|Default|GetToggleBox_English))))
  (Utilities|Array|Add (Variables|Default|GetToggleBoxes) _asbp_toggle_box)
  (bind _asbp_toggle_box_2 (Utilities|Casting|CastToBP_ToggleBox (Variables|/Script/Engine.ChildActorComponent|GetChildActor (Variables|Default|GetToggleBox_Dutch))))
  (Utilities|Array|Add (Variables|Default|GetToggleBoxes) _asbp_toggle_box_2)
  (bind _asbp_toggle_box_3 (Utilities|Casting|CastToBP_ToggleBox (Variables|/Script/Engine.ChildActorComponent|GetChildActor (Variables|Default|GetToggleBox_French))))
  (Utilities|Array|Add (Variables|Default|GetToggleBoxes) _asbp_toggle_box_3)
  (for _array_element (Variables|Default|GetToggleBoxes)
    (if (Variables|/Game/Blueprints/InteractiveElements/3DUI/BP_ToggleBox.BP_ToggleBox_C|GetIsActive _array_element)
      (Transformation|SetWorldScale3D (Variables|/Script/Engine.StaticMeshActor|GetStaticMeshComponent _array_element) "1.150000,1.150000,1.150000"))))

(event Collision|EventActorBeginOverlap
  (params (OtherActor :type Actor%20Object%20Reference)))

(event EventTick
  (params (DeltaSeconds :type Float%20%28single-precision%29))
  (CallFunction|CheckChangedToggleBoxes))

(fn ConstructionScript)

(fn CheckChangedToggleBoxes
  (Utilities|FlowControl|Sequence
    (:then_0
      (for (_array_element _array_index) (Variables|Default|GetToggleBoxes)
        (if (Variables|/Game/Blueprints/InteractiveElements/3DUI/BP_ToggleBox.BP_ToggleBox_C|GetHasChanged _array_element)
          (LocalVariables|SetChangedIndex _array_index))))
    (:then_1
      (if (!= (LocalVariables|GetChangedIndex) -1)
        (Utilities|FlowControl|Sequence
          (:then_0
            (for (_array_element_2 _array_index_2) (Variables|Default|GetToggleBoxes)
              (Utilities|IsValid _array_element_2
                (:Is%20Valid
                  (if (!= _array_index_2 (LocalVariables|GetChangedIndex))
                    (Default|Disable _array_element_2)
                    (Transformation|SetWorldScale3D (Variables|/Script/Engine.StaticMeshActor|GetStaticMeshComponent _array_element_2) "1.000000,1.000000,1.000000"))))))
          (:then_1
            (Utilities|IsValid (Utilities|Array|Get(acopy) (Variables|Default|GetToggleBoxes) (LocalVariables|GetChangedIndex))
              (:Is%20Valid
                (Default|Enable (Utilities|Array|Get(acopy) (Variables|Default|GetToggleBoxes) (LocalVariables|GetChangedIndex)))
                (Transformation|SetWorldScale3D (Variables|/Script/Engine.StaticMeshActor|GetStaticMeshComponent (Utilities|Array|Get(acopy) (Variables|Default|GetToggleBoxes) (LocalVariables|GetChangedIndex))) "1.150000,1.150000,1.150000")))))))))