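; BP_ToggleBox is an interactive 3D UI toggle for switching the game's language.
; Pickup presses or overlaps from the pawn's hand spheres set HasChanged, with overlaps also showing a confirmation text.
; Enable applies its Language culture without saving and Tick keeps the dynamic material glowing while active; Disable dims it.
; A separate Squesh event animates mesh scale through a timeline, and other interaction handlers are stubs.
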(event OnComponentBeginOverlap(StaticMeshComponent)
  (params (OverlappedComponent :type Primitive%20Component%20Object%20Reference) (OtherActor :type Actor%20Object%20Reference) (OtherComp :type Primitive%20Component%20Object%20Reference) (OtherBodyIndex :type Integer) (bFromSweep :type Boolean) (SweepResult :type Hit%20Result%20Structure%20%28by%20ref%29))
  (bind _asbp_base_pawn (Utilities|Casting|CastToBP_BasePawn OtherActor))
  (Utilities|IsValid (Variables|/Script/GiantHouseDEV.BasePawn|GetpHandSphereL _asbp_base_pawn)
    (:Is%20Valid
      (Utilities|IsValid (Variables|/Script/GiantHouseDEV.BasePawn|GetpHandSphereR _asbp_base_pawn)
        (:Is%20Valid
          (if (or (== (Variables|/Script/GiantHouseDEV.BasePawn|GetpHandSphereL _asbp_base_pawn) OtherComp) (== (Variables|/Script/GiantHouseDEV.BasePawn|GetpHandSphereR _asbp_base_pawn) OtherComp))
            (CallFunction|PickupActor)
            (bind _asbp_game_instance (Utilities|Casting|CastToBP_GameInstance (Game|GetGameInstance)))
            (Default|SetSpringTextwithAliveDelay (Variables|/Game/Blueprints/BP_GameInstance.BP_GameInstance_C|GetBasePawn _asbp_game_instance) "YOU CHANGED THE LANGUAGE" 0.5 5.0)))))))

(event Custom|PickupActor
  (params (NewInteractor :type World%20Interactor%20Object%20Reference))
  (Variables|Default|SetHasChanged true))

(event Custom|Disable
  (Variables|Default|SetHasChanged false)
  (Variables|Default|SetIsActive false)
  (Rendering|Material|SetScalarParameterValue (Variables|Default|GetToggleBoxMat) "EmissiveIntensity" 0.2 :!class /Script/Engine.MaterialInstanceDynamic))

(event Custom|Squesh
  (bind _scale (Timeline|Timeline_0 PlayFromStart)
    (:Update
      (Transformation|SetWorldScale3D (Variables|Debug|GetStaticMeshComponent) _scale))))

(event Custom|Enable
  (Variables|Default|SetHasChanged false)
  (Variables|Default|SetIsActive true)
  (Class|KismetInternationalizationLibrary|SetCurrentCulture (Variables|Default|GetLanguage)))

(event EventBeginPlay
  (bind _staticmeshcomponent (Variables|Debug|GetStaticMeshComponent))
  (bind _returnvalue (Rendering|Material|CreateDynamicMaterialInstance _staticmeshcomponent 0 (Rendering|Material|GetMaterial _staticmeshcomponent 0) "None" :!class /Script/Engine.PrimitiveComponent))
  (Variables|Default|SetToggleBoxMat _returnvalue))

(event EventTick
  (params (DeltaSeconds :type Float%20%28single-precision%29))
  (if (Variables|Default|GetIsActive)
    (Rendering|Material|SetScalarParameterValue (Variables|Default|GetToggleBoxMat) "EmissiveIntensity" 5.0 :!class /Script/Engine.MaterialInstanceDynamic)))

(fn ConstructionScript)

(fn GetClosestComponentData
  (params (interactor :type World%20Interactor%20Object%20Reference))
  (return (.OutPointOnBody (Collision|GetClosestPointonCollision (Variables|Debug|GetStaticMeshComponent) (Transformation|GetWorldLocation interactor) "None")) 5 (Variables|Debug|GetStaticMeshComponent)))

(fn OnDrag
  (params (interactor :type World%20Interactor%20Object%20Reference))
  (return false))

(fn OnDragStart
  (params (interactor :type World%20Interactor%20Object%20Reference))
  (return false))

(fn OnDragStop
  (params (interactor :type World%20Interactor%20Object%20Reference))
  (return false))

(fn OnHover
  (params (interactor :type World%20Interactor%20Object%20Reference))
  (return false))

(fn OnHoveredComponentChanged
  (params (interactor :type World%20Interactor%20Object%20Reference) (oldComponent :type Scene%20Component%20Object%20Reference) (newComponent :type Scene%20Component%20Object%20Reference))
  (return false))

(fn OnPickupPressed
  (params (interactor :type World%20Interactor%20Object%20Reference))
  (Utilities|IsValid interactor
    (:Is%20Valid
      (CallFunction|PickupActor interactor)
      (return false))))

(fn OnPickupReleased
  (params (interactor :type World%20Interactor%20Object%20Reference))
  (return false))

(fn OnUnhover
  (params (interactor :type World%20Interactor%20Object%20Reference))
  (return false))

(fn OnUsePressed
  (params (interactor :type World%20Interactor%20Object%20Reference))
  (return false))

(fn OnUseReleased
  (params (interactor :type World%20Interactor%20Object%20Reference))
  (return false))