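; Washing machine hazard that traps and drowns the player, then loads the death scene with a WashMachine option.
; The start trigger marks the pawn as dying and teleports it inside behind a camera fade.
; Tick then steps through staged flags: timelines close the door and raise the water, then a timer fades out to death.
; Underwater overlap adds sound and a washing material to the MainPV-tagged post-process volume.
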(event OnComponentBeginOverlap(EventStartTrigger)
  (params (OverlappedComponent :type Primitive%20Component%20Object%20Reference) (OtherActor :type Actor%20Object%20Reference) (OtherComp :type Primitive%20Component%20Object%20Reference) (OtherBodyIndex :type Integer) (bFromSweep :type Boolean) (SweepResult :type Hit%20Result%20Structure%20%28by%20ref%29))
  (bind _returnvalue (Game|GetPlayerCameraManager 0))
  (bind _returnvalue_2 (Actor|GetAttachParentActor OtherActor))
  (bind _teleportlocation (Variables|Default|GetTeleportLocation))
  (bind _returnvalue_3 (Transformation|GetWorldTransform _teleportlocation))
  (bind (_location _rotation) (Math|Transform|BreakTransform _returnvalue_3))
  ;[1 1 1] Start Event
  (bind _asbp_game_instance (Utilities|Casting|CastToBP_GameInstance (Game|GetGameInstance)))
  (if (not (Variables|/Game/Blueprints/BP_GameInstance.BP_GameInstance_C|GetbFinishedWashingMachine _asbp_game_instance))
    (Utilities|IsValid _returnvalue_2
      (:Is%20Valid
        (Utilities|Casting|CastToBP_BasePawn _returnvalue_2))
      (:Is%20Not%20Valid
        (Utilities|Casting|CastToBP_BasePawn OtherActor)))
    (bind _asbp_game_instance_2 (Utilities|Casting|CastToBP_GameInstance (Game|GetGameInstance)))
    (if (not (Class|BasePawn|IsDying (Variables|/Game/Blueprints/BP_GameInstance.BP_GameInstance_C|GetBasePawn _asbp_game_instance_2)))
      (bind _asbp_game_instance_3 (Utilities|Casting|CastToBP_GameInstance (Game|GetGameInstance)))
      (Class|BasePawn|SetDying (Variables|/Game/Blueprints/BP_GameInstance.BP_GameInstance_C|GetBasePawn _asbp_game_instance_3) true)
      (Default|SavePawnLocation _asbp_game_instance)
      (CameraFades|StartCameraFade :self _returnvalue :ToAlpha 1.0 :Duration 1.0 :bHoldWhenFinished true)
      (Utilities|FlowControl|Delay 1.0)
      (Transformation|SetActorLocation (Variables|/Game/Blueprints/BP_GameInstance.BP_GameInstance_C|GetBasePawn _asbp_game_instance) _location false false)
      (Pawn|SetControlRotation (Pawn|GetController (Variables|/Game/Blueprints/BP_GameInstance.BP_GameInstance_C|GetBasePawn _asbp_game_instance)) _rotation)
      (CameraFades|StartCameraFade :self _returnvalue :FromAlpha 1.0 :Duration 1.0)
      (Variables|Default|SetbInsideMachine true)
      (Default|DisableWashingMachine _asbp_game_instance))))

(event OnComponentBeginOverlap(UnderwaterC)
  (params (OverlappedComponent :type Primitive%20Component%20Object%20Reference) (OtherActor :type Actor%20Object%20Reference) (OtherComp :type Primitive%20Component%20Object%20Reference) (OtherBodyIndex :type Integer) (bFromSweep :type Boolean) (SweepResult :type Hit%20Result%20Structure%20%28by%20ref%29))
  ;[1 1 1] drown
  (Utilities|Casting|CastToBP_BasePawn OtherActor)
  (Utilities|Casting|CastToSphereComponent OtherComp)
  (Audio|Components|Audio|FadeIn (Variables|Default|GetUnderwater) 0.5 1.0 0.0 :!class /Script/Engine.AudioComponent)
  (Utilities|Array|Add (Utilities|Struct|BreakWeightedBlendables (Utilities|Struct|BreakPostProcessSettings (Variables|/Script/Engine.PostProcessVolume|GetSettings (Variables|Default|GetPPV)))) (Utilities|Struct|MakeWeightedBlendable 1.0 (Variables|Default|GetPPMAt))))

(event Custom|CloseDoor
  (bind _door (Variables|Default|GetDoor))
  ;[1 1 1] closing door
  (bind _driver (Timeline|Timeline_DoorClose Play)
    (:Update
      (Transformation|SetRelativeRotation _door (Math|Rotator|Lerp(Rotator) (Variables|/Script/Engine.SceneComponent|GetRelativeRotation _door) "0, 0, 0" _driver true) false false))
    (:Finished
      (CallFunction|StopCloseDoor)
      (Variables|Default|SetbDoorIsClosed true))
    (:PlaySoundEvent
      (Audio|Components|Audio|Play (Variables|Default|GetDoorClose) 0.0))))

(event Custom|Start%20Fill
  (bind _waterfill (Variables|Default|GetWaterFill))
  (bind _waterlevel (Variables|Default|GetWaterLevel))
  ;[1 1 1] Fill
  (if (Audio|Components|Audio|IsPlaying _waterfill)
    (bind _driver (Timeline|Timeline_Fill Play)
      (:Update
        (Transformation|SetRelativeLocation _waterlevel (Math|Vector|Lerp(Vector) (Variables|/Script/Engine.SceneComponent|GetRelativeLocation _waterlevel) (Variables|/Script/Engine.SceneComponent|GetRelativeLocation (Variables|Default|GetWaterRiseLimit)) _driver) false false))
      (:Finished
        (CallFunction|StopFill)
        (Variables|Default|SetbIsFilled true)))
    (else
      (Audio|Components|Audio|FadeIn _waterfill 0.5 1.0 0.0 :!class /Script/Engine.AudioComponent)
      (Timeline|Timeline_Fill Play))))

(event Custom|Stop%20Fill
  (bind _waterfill (Variables|Default|GetWaterFill))
  (bind _underwater (Variables|Default|GetUnderwater))
  (bind _waterlevel (Variables|Default|GetWaterLevel))
  ;[1 1 1] Fill
  (if (Audio|Components|Audio|IsPlaying _waterfill)
    (Audio|Components|Audio|FadeOut _waterfill 0.5 0.0 :!class /Script/Engine.AudioComponent))
  (if (Audio|Components|Audio|IsPlaying _underwater)
    (bind _driver (Timeline|Timeline_Fill Stop)
      (:Update
        (Transformation|SetRelativeLocation _waterlevel (Math|Vector|Lerp(Vector) (Variables|/Script/Engine.SceneComponent|GetRelativeLocation _waterlevel) (Variables|/Script/Engine.SceneComponent|GetRelativeLocation (Variables|Default|GetWaterRiseLimit)) _driver) false false))
      (:Finished
        (CallFunction|StopFill)
        (Variables|Default|SetbIsFilled true)))
    (else
      (Audio|Components|Audio|FadeIn _underwater 0.5 1.0 0.0 :!class /Script/Engine.AudioComponent)
      (Timeline|Timeline_Fill Stop))))

(event Custom|StopCloseDoor
  (bind _door (Variables|Default|GetDoor))
  ;[1 1 1] closing door
  (bind _driver (Timeline|Timeline_DoorClose Stop)
    (:Update
      (Transformation|SetRelativeRotation _door (Math|Rotator|Lerp(Rotator) (Variables|/Script/Engine.SceneComponent|GetRelativeRotation _door) "0, 0, 0" _driver true) false false))
    (:Finished
      (CallFunction|StopCloseDoor)
      (Variables|Default|SetbDoorIsClosed true))
    (:PlaySoundEvent
      (Audio|Components|Audio|Play (Variables|Default|GetDoorClose) 0.0))))

(event Custom|ResetHazard
  ;[1 1 1] Start Event
)

(event EventBeginPlay
  ;[1 1 1] Find Volumes
  (bind _outactors (Actor|GetAllActorswithTag "MainPV"))
  (bind _aspost_process_volume (Utilities|Casting|CastToPostProcessVolume (Utilities|Array|Get(acopy) _outactors)))
  (Variables|Default|SetPPV _aspost_process_volume)
  (bind _returnvalue (Rendering|Material|CreateDynamicMaterialInstance "/Game/Materials/Post_Washing_Inst.Post_Washing_Inst" "None" :!class /Script/Engine.KismetMaterialLibrary))
  (Variables|Default|SetPPMAt _returnvalue)
  (Audio|Components|Audio|Stop (Variables|Default|GetWaterFill))
  (Audio|Components|Audio|Stop (Variables|Default|GetDoorClose))
  (Audio|Components|Audio|Stop (Variables|Default|GetUnderwater)))

(event Collision|EventActorBeginOverlap
  (params (OtherActor :type Actor%20Object%20Reference)))

(event EventTick
  (params (DeltaSeconds :type Float%20%28single-precision%29))
  ;[1 1 1] Check which stage
  (if (Variables|Default|GetbInsideMachine)
    (if (Variables|Default|GetbDoorIsClosed)
      (if (Variables|Default|GetbIsFilled)
        (bind _output_get (Variables|Default|SetDeathTimer (+ DeltaSeconds (Variables|Default|GetDeathTimer))))
        (if (> _output_get (Variables|Default|GetDeathTimerMax))
          (CallFunction|ResetHazard)
          (bind _asbp_game_instance (Utilities|Casting|CastToBP_GameInstance (Game|GetGameInstance)))
          (Variables|/Game/Blueprints/BP_GameInstance.BP_GameInstance_C|SetLevelLoadOptions _asbp_game_instance "WashMachine")
          (Game|OpenLevel(byName) "MAP_PlayerDeadScene")
          (else
            (Utilities|FlowControl|DoOnce false
              (:Completed
                (CameraFades|StartCameraFade :self (Game|GetPlayerCameraManager 0) :ToAlpha 1.0 :Duration (Variables|Default|GetDeathTimerMax) :bShouldFadeAudio true :bHoldWhenFinished true)))))
        (else
          (CallFunction|StartFill)))
      (else
        (CallFunction|CloseDoor)))))

(fn ConstructionScript)