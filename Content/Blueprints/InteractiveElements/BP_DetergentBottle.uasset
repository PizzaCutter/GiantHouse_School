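; Pickup detergent bottle hazard that kills the player who drinks from it.
; Pressing pickup while a pawn overlaps the cap collision hides the cap and marks it open.
; Once open, Tick traces from the cap for a pawn sphere at or below bottle height to detect drinking.
; Drinking triggers sounds, splash and a post-process material, saves pawn location, then fades to the death scene using GameInstance timings.
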(event EventBeginPlay
  (bind _returnvalue (Rendering|Material|CreateDynamicMaterialInstance "/Game/Materials/Post_Washing_Inst.Post_Washing_Inst" "None" :!class /Script/Engine.KismetMaterialLibrary))
  (Variables|Default|SetPPMat _returnvalue)
  (bind _outactors (Actor|GetAllActorswithTag "MainPV"))
  (bind _aspost_process_volume (Utilities|Casting|CastToPostProcessVolume (Utilities|Array|Get(acopy) _outactors)))
  (Variables|Default|SetPPVol _aspost_process_volume))

(event Collision|EventActorBeginOverlap
  (params (OtherActor :type Actor%20Object%20Reference)))

(event EventTick
  (params (DeltaSeconds :type Float%20%28single-precision%29))
  (bind _cap (Variables|Default|GetCap))
  (bind _returnvalue (Transformation|GetWorldLocation _cap))
  (if (Variables|Default|GetbCapOff)
    (bind (_outhit _returnvalue_2) (Collision|LineTraceForObjects _returnvalue (+ _returnvalue (* (Math|Vector|GetForwardVector (Variables|Default|GetCap)) (Variables|Default|GetRange))) (Utilities|Array|MakeArray "ObjectTypeQuery3") false 0 "None" true "(R=1.000000,G=0.000000,B=0.000000,A=1.000000)" "(R=0.000000,G=1.000000,B=0.000000,A=1.000000)" 0.0))
    (bind _assphere_collision (Utilities|Casting|CastToSphereComponent (.hitcomponent _outhit)))
    (if _returnvalue_2
      (if (<= (.Z (Math|Vector|BreakVector (Transformation|GetWorldLocation _assphere_collision))) (.z (Transformation|GetWorldLocation (Variables|Default|GetStaticMeshComponent))))
        (Utilities|FlowControl|DoOnce false :!label _label
          (:Completed
            (Development|PrintString "DRINKING FROM BOTTLE" true false "(R=0.000000,G=0.660000,B=1.000000,A=1.000000)" 0.5)
            (Audio|PlaySoundatLocation "/Game/Audio/SFX/SFX_Splash_Pot.SFX_Splash_Pot" (Transformation|GetActorLocation) "0, 0, 0" 1.0 1.0 0.0 0 0 0)
            (Audio|SpawnSound2D "/Game/Audio/SFX/SFX_BabyHurt.SFX_BabyHurt" 1.0 1.0 0.0 0)
            (Components|Activation|Activate (Variables|Default|GetSplash) false)
            (Utilities|Array|Add (Utilities|Struct|BreakWeightedBlendables (Utilities|Struct|BreakPostProcessSettings (Variables|/Script/Engine.PostProcessVolume|GetSettings (Variables|Default|GetPPVol)))) (Utilities|Struct|MakeWeightedBlendable 1.0 (Variables|Default|GetPPMat)))
            (bind _asbp_game_instance (Utilities|Casting|CastToBP_GameInstance (Game|GetGameInstance)))
            (Default|SavePawnLocation _asbp_game_instance)
            (Utilities|FlowControl|Delay (Variables|/Game/Blueprints/BP_GameInstance.BP_GameInstance_C|GetHazardKillTime _asbp_game_instance))
            (CameraFades|StartCameraFade :self (Game|GetPlayerCameraManager 0) :ToAlpha 1.0 :Duration (Variables|/Game/Blueprints/BP_GameInstance.BP_GameInstance_C|GetFadeTime _asbp_game_instance))
            (Utilities|FlowControl|Delay (Variables|/Game/Blueprints/BP_GameInstance.BP_GameInstance_C|GetFadeTime _asbp_game_instance))
            (Variables|/Game/Blueprints/BP_GameInstance.BP_GameInstance_C|SetLevelLoadOptions _asbp_game_instance "Detergent")
            (Game|OpenLevel(byName) "MAP_PlayerDeadScene")))
        (else
          (goto _label Reset))))))

(fn ConstructionScript
  (|CallParentFunction))

(fn OnPickupPressed
  (params (interactor :type World%20Interactor%20Object%20Reference))
  (|CallParentFunction interactor)
  (if (Variables|Default|GetbCapOff)
    (return false)
    (else
      (if (< 0 (Utilities|Array|Length (Collision|GetOverlappingActors (Variables|Default|GetCapCollision) "/Game/Blueprints/Gameplay/BP_BasePawn.BP_BasePawn_C" :!class /Script/Engine.PrimitiveComponent)))
        (Rendering|SetVisibility (Variables|Default|GetCapMesh) false false)
        (Variables|Default|SetbCapOff true))
      (return false))))

(fn OnPickupReleased
  (params (interactor :type World%20Interactor%20Object%20Reference))
  (bind _returnvalue (|CallParentFunction interactor))
  (return _returnvalue))