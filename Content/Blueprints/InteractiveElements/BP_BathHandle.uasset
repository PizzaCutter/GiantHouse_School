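; Bath tap handle that detects when it has been turned open and starts the bathtub water.
; While not disabled, Tick compares the yaw of PDoorRotator against the ATapOpen reference, with SmallerThen choosing the comparison direction.
; Crossing that threshold fires SpawnWater through a DoOnce.
; SpawnWater prints a debug message, disables every BP_SinkHandle and calls Start on the first BP_BathtubWater found in the level.
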(event Custom|SpawnWater
  (Utilities|FlowControl|Sequence
    (:then_0
      (Development|PrintString "TAP OPENED"))
    (:then_1
      (bind _outactors (Actor|GetAllActorsOfClass "/Game/Blueprints/InteractiveElements/BP_SinkHandle.BP_SinkHandle_C"))
      (for _array_element _outactors
        (Variables|/Game/Blueprints/InteractiveElements/BP_SinkHandle.BP_SinkHandle_C|SetbDisable _array_element true)))
    (:then_2
      (bind _outactors_2 (Actor|GetAllActorsOfClass "/Game/Blueprints/BP_BathtubWater.BP_BathtubWater_C"))
      (Default|Start (Utilities|Array|Get(acopy) _outactors_2)))))

(event EventTick
  (params (DeltaSeconds :type Float%20%28single-precision%29))
  (if (not (Variables|Default|GetbDisable))
    (if (Variables|Default|GetbSmallerThen)
      (Utilities|FlowControl|Sequence
        (:then_0
          (if (<= (.yaw (Variables|/Script/Engine.SceneComponent|GetRelativeRotation (Variables|Default|GetA_TapOpen))) (.yaw (Variables|/Script/Engine.SceneComponent|GetRelativeRotation (Variables|Default|GetpDoorRotator))))
            (Utilities|FlowControl|DoOnce false
              (:Completed
                (CallFunction|SpawnWater)))))
        (:then_1
          (if (> (.yaw (Variables|/Script/Engine.SceneComponent|GetRelativeRotation (Variables|Default|GetA_TapOpen))) (.yaw (Variables|/Script/Engine.SceneComponent|GetRelativeRotation (Variables|Default|GetpDoorRotator))))
            _)))
      (else
        (Utilities|FlowControl|Sequence
          (:then_0
            (if (>= (.yaw (Variables|/Script/Engine.SceneComponent|GetRelativeRotation (Variables|Default|GetA_TapOpen))) (.yaw (Variables|/Script/Engine.SceneComponent|GetRelativeRotation (Variables|Default|GetpDoorRotator))))
              (Utilities|FlowControl|DoOnce false
                (:Completed
                  (CallFunction|SpawnWater)))))
          (:then_1
            (if (< (.yaw (Variables|/Script/Engine.SceneComponent|GetRelativeRotation (Variables|Default|GetA_TapOpen))) (.yaw (Variables|/Script/Engine.SceneComponent|GetRelativeRotation (Variables|Default|GetpDoorRotator))))
              _)))))))

(fn ConstructionScript)