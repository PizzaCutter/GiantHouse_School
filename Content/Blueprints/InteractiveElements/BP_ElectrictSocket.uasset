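; Electric socket hazard that electrocutes the VR player when either hand sphere enters its electrify collider.
; A one-shot overlap marks the pawn as dying, starts its electrification and stores both motion controller locations, which Tick reapplies to pin the hands in place.
; It saves the pawn location through the game instance, waits the hazard kill time, fades to white and opens the player-dead map tagged "Socket".
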(event OnComponentBeginOverlap(BC_ElectrifyCollider)
  (params (OverlappedComponent :type Primitive%20Component%20Object%20Reference) (OtherActor :type Actor%20Object%20Reference) (OtherComp :type Primitive%20Component%20Object%20Reference) (OtherBodyIndex :type Integer) (bFromSweep :type Boolean) (SweepResult :type Hit%20Result%20Structure%20%28by%20ref%29))
  (bind _asbp_base_pawn (Utilities|Casting|CastToBP_BasePawn OtherActor))
  (bind _output_get (Variables|Default|SetBasePawn _asbp_base_pawn))
  (if (not (Class|BasePawn|IsDying _output_get))
    (Utilities|IsValid (Variables|/Script/GiantHouseDEV.BasePawn|GetpHandSphereL (Variables|Default|GetBasePawn))
      (:Is%20Valid
        (Utilities|IsValid (Variables|/Script/GiantHouseDEV.BasePawn|GetpHandSphereR (Variables|Default|GetBasePawn))
          (:Is%20Valid
            (if (or (== (Variables|/Script/GiantHouseDEV.BasePawn|GetpHandSphereL (Variables|Default|GetBasePawn)) OtherComp) (== (Variables|/Script/GiantHouseDEV.BasePawn|GetpHandSphereR (Variables|Default|GetBasePawn)) OtherComp))
              (bind _asbp_game_instance (Utilities|Casting|CastToBP_GameInstance (Game|GetGameInstance)))
              (if (not (Class|BasePawn|IsDying (Variables|/Game/Blueprints/BP_GameInstance.BP_GameInstance_C|GetBasePawn _asbp_game_instance)))
                (Utilities|FlowControl|DoOnce false
                  (:Completed
                    (Utilities|FlowControl|Sequence
                      (:then_0
                        (Variables|Default|SetControllerLocationL (Transformation|GetWorldLocation (Variables|/Script/GiantHouseDEV.BasePawn|GetpMotionControllerL (Variables|Default|GetBasePawn))))
                        (Variables|Default|SetControllerLocationR (Transformation|GetWorldLocation (Variables|/Script/GiantHouseDEV.BasePawn|GetpMotionControllerR (Variables|Default|GetBasePawn))))
                        (Variables|Default|SetbStartedElectrocuting true))
                      (:then_1
                        (CallFunction|Electrecute))
                      (:then_2
                        (bind _asbp_game_instance_2 (Utilities|Casting|CastToBP_GameInstance (Game|GetGameInstance)))
                        (Class|BasePawn|SetDying (Variables|/Game/Blueprints/BP_GameInstance.BP_GameInstance_C|GetBasePawn _asbp_game_instance_2) true)))))))))))))

(event Custom|Electrecute
  (Default|StartElectrification (Variables|/Game/Blueprints/BP_GameInstance.BP_GameInstance_C|GetBasePawn (.AsBP%20Game%20Instance (Utilities|Casting|CastToBP_GameInstance (Game|GetGameInstance)))) "NewEnumerator0")
  (bind _asbp_game_instance (Utilities|Casting|CastToBP_GameInstance (Game|GetGameInstance)))
  (Default|SavePawnLocation _asbp_game_instance)
  (Utilities|FlowControl|Delay (Variables|/Game/Blueprints/BP_GameInstance.BP_GameInstance_C|GetHazardKillTime _asbp_game_instance))
  (CameraFades|StartCameraFade (Game|GetPlayerCameraManager 0) 0.0 1.0 (Variables|/Game/Blueprints/BP_GameInstance.BP_GameInstance_C|GetFadeTime _asbp_game_instance) "(R=1.000000,G=1.000000,B=1.000000,A=1.000000)" false true)
  (Utilities|FlowControl|Delay (Variables|/Game/Blueprints/BP_GameInstance.BP_GameInstance_C|GetFadeTime _asbp_game_instance))
  (Variables|/Game/Blueprints/BP_GameInstance.BP_GameInstance_C|SetLevelLoadOptions _asbp_game_instance "Socket")
  (Game|OpenLevel(byName) "MAP_PlayerDeadScene"))

(event EventTick
  (params (DeltaSeconds :type Float%20%28single-precision%29))
  (if (Variables|Default|GetbStartedElectrocuting)
    (Transformation|SetWorldLocation (Variables|/Script/GiantHouseDEV.BasePawn|GetpMotionControllerL (Variables|Default|GetBasePawn)) (Variables|Default|GetControllerLocationL) false true)
    (Transformation|SetWorldLocation (Variables|/Script/GiantHouseDEV.BasePawn|GetpMotionControllerR (Variables|Default|GetBasePawn)) (Variables|Default|GetControllerLocationR) false true)))

(fn ConstructionScript)